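; Attack instance actor that validates victims and applies hit damage and feedback.
; ShouldHitActor extends ShouldImpactActor with a TeamID check, though it rejects every hit when ShouldFriendlyFire is true.
; HitActor calls ImpactActor, then triggers component-based hitstop and flash, knockback impulse with fixed upward lift, particles, audio and camera shake at the owner's camera.
; CalcDamageBP simply returns DamageModifier.
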(fn `ApplyHitFlash`
  (params (Actor :type "Actor Object Reference") (Duration :type "Float (single-precision)"))
  (bind _returnvalue (`self.GetComponentByClass` (`local.Actor`) "/Game/NecroPixelsContent/Components/Pawns/HitFlashComponent.HitFlashComponent_C"))
  (`/Engine/EditorBlueprintResources/StandardMacros.IsValid` (`local.Actor`)
    (:`Is Valid`
      (`/Engine/EditorBlueprintResources/StandardMacros.IsValid` _returnvalue
        (:`Is Valid`
          (`/Game/NecroPixelsContent/Components/Pawns/HitFlashComponent.StartFlash` _returnvalue (`local.Duration`)))))))

(fn `ApplyHitstop`
  (params (Actor :type "Actor Object Reference") (Duration :type "Float (single-precision)"))
  (bind _returnvalue (`self.GetComponentByClass` (`local.Actor`) "/Game/NecroPixelsContent/Components/Pawns/HitstopComponent.HitstopComponent_C"))
  (`/Engine/EditorBlueprintResources/StandardMacros.IsValid` (`local.Actor`)
    (:`Is Valid`
      (`/Engine/EditorBlueprintResources/StandardMacros.IsValid` _returnvalue
        (:`Is Valid`
          (`/Game/NecroPixelsContent/Components/Pawns/HitstopComponent.StartHitStop` _returnvalue (`local.Duration`)))))))

(fn `ApplyKnockback`
  (params (Actor :type "Actor Object Reference"))
  (locals (KnockbackDirection :type "Vector Structure" :default (0.0 0.0 0.0)))
  (bind _returnvalue (`self.GetComponentByClass` (`local.Actor`) "/Script/Engine.CharacterMovementComponent"))
  (`/Engine/EditorBlueprintResources/StandardMacros.IsValid` (`local.Actor`)
    (:`Is Valid`
      (`/Engine/EditorBlueprintResources/StandardMacros.IsValid` _returnvalue
        (:`Is Valid`
          (set `local.KnockbackDirection` (`KismetMathLibrary.Normal` (- (`self.K2_GetActorLocation` (`local.Actor`)) (`self.K2_GetActorLocation`))))
          (`CharacterMovementComponent.AddImpulse` _returnvalue (+ (* (`local.KnockbackDirection`) (`self.KnockbackForce`)) (* (0.0 0.0 1.0) 1000.0)) false))))))

(fn `CalcDamage_BP`
  (returns (ReturnValue :type "Float (single-precision)"))
  (return (`self.DamageModifier`)))

(fn `CameraShake`
  (bind _returnvalue (`self.GetOwner`))
  (bind _returnvalue_2 (`self.GetComponentByClass` _returnvalue "/Script/Engine.CameraComponent"))
  (`/Engine/EditorBlueprintResources/StandardMacros.IsValid` _returnvalue
    (:`Is Valid`
      (`/Engine/EditorBlueprintResources/StandardMacros.IsValid` _returnvalue_2
        (:`Is Valid`
          (`GameplayStatics.PlayWorldCameraShake` (`self.ImpactCameraShake`) (`SceneComponent.K2_GetComponentLocation` _returnvalue_2) 0.0 500.0))))))

(fn `HitActor`
  (params (Victim :type "Actor Object Reference"))
  ;[1 1 1] Apply damage add actor to array
  (`self.ImpactActor` Victim)
  (`|ExecutionSequence`
    (:`then_0`
      ;[1 1 1] Hitstop Effect
      (if (> (`self.HitstopDuration`) 0.0)
        (`self.ApplyHitstop` (`local.Victim`) (`self.HitstopDuration`))
        (`self.ApplyHitstop` (`self.GetOwner`) (`self.HitstopDuration`))
        (`self.ApplyHitFlash` (`local.Victim`) (`self.HitstopDuration`))))
    (:`then_1`
      ;[1 1 1] Knockback
      (if (> (`self.KnockbackForce`) 0.0)
        (`self.ApplyKnockback` (`local.Victim`))))
    (:`then_2`
      ;[1 1 1] Impact Feedback
      (`self.SpawnHitParticle` (`local.Victim`))
      (`AudioComponent.Play` (`self.Impact_Audio`) 0.0))
    (:`then_3`
      ;[1 1 1] Player User Feedback
      (`self.CameraShake`))))

(fn `ShouldHitActor`
  (params (Actor :type "Actor Object Reference"))
  (returns (bShouldHitActor :type Boolean))
  (locals (VictimTeam :type "/Game/NecroPixelsContent/Components/Pawns/TeamComponent Object Reference") (OwnerTeam :type "/Game/NecroPixelsContent/Components/Pawns/TeamComponent Object Reference"))
  ;[1 1 1] Should Self Harm?
  (if (`self.ShouldImpactActor` (`local.Actor`))
    ;[1 1 1] Comment
    (if (not (`self.bShouldFriendlyFire`))
      (bind _output_get (set `local.VictimTeam` (`self.GetComponentByClass` (`local.Actor`) "/Game/NecroPixelsContent/Components/Pawns/TeamComponent.TeamComponent_C")))
      (`/Engine/EditorBlueprintResources/StandardMacros.IsValid` _output_get
        (:`Is Valid`
          (bind _output_get_2 (set `local.OwnerTeam` (`self.GetComponentByClass` (`self.GetOwner`) "/Game/NecroPixelsContent/Components/Pawns/TeamComponent.TeamComponent_C")))
          (`/Engine/EditorBlueprintResources/StandardMacros.IsValid` _output_get_2
            (:`Is Valid`
              (if (!= (`/Game/NecroPixelsContent/Components/Pawns/TeamComponent.TeamID` (`local.VictimTeam`)) (`/Game/NecroPixelsContent/Components/Pawns/TeamComponent.TeamID` (`local.OwnerTeam`)))
                ;[0 1 0.135] Yes.
                (return true)
                (else
                  _)))
            (:`Is Not Valid`
              (return true))))
        (:`Is Not Valid`
          (return true)))))
  ;[1 0 0] No.
  (return false))

(fn `SpawnHitParticle`
  (params (Actor :type "Actor Object Reference"))
  (`NiagaraFunctionLibrary.SpawnSystemAttached` (`self.ImpactParticle`) (`Actor.RootComponent` Actor) "None" (0.0 0.0 0.0) (struct) "SnapToTargetIncludingScale" true))

(fn `UserConstructionScript`)