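; BP_Forest fills a box-sized area with a staggered grid of tree sprites, built in the construction script.
; It clears the PaperGroupedSprite, then loops over columns and rows derived from the box extent and placement width and height, adding one TreeSprite instance per cell.
; Odd columns shift by half a row, and Z varies by row and column parity to layer the rotated sprites.
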(fn `InitializeForestTiles`
  (locals (LocX :type Integer) (LocY :type Integer))
  (bind _locy (`local.LocY`))
  (bind _returnvalue (mod (`local.LocX`) 2))
  (bind (_boxextent_x _boxextent_y) (`KismetMathLibrary.BreakVector` (`BoxComponent.BoxExtent` (`self.Box`))))
  (bind _returnvalue_2 (`KismetMathLibrary.FTrunc` (/ _boxextent_y (`self.PlacementHeight`))))
  (bind _returnvalue_3 (`KismetMathLibrary.FTrunc` (/ _boxextent_x (`self.PlacementWidth`))))
  (`PaperGroupedSpriteComponent.ClearInstances` (`self.PaperGroupedSprite`))
  (for _index (range (- 0 _returnvalue_3) (+ _returnvalue_3 1))
    (set `local.LocX` _index)
    (for _index_2 (range (- 0 _returnvalue_2) (+ _returnvalue_2 1))
      (set `local.LocY` _index_2)
      (`PaperGroupedSpriteComponent.AddInstance` (`self.PaperGroupedSprite`) (`KismetMathLibrary.MakeTransform` (`KismetMathLibrary.MakeVector` (* (`local.LocX`) (`self.PlacementWidth`)) (+ (* _locy (`self.PlacementHeight`)) (* (`self.PlacementHeight`) 0.5 _returnvalue)) (+ (* _locy 1.1) _returnvalue)) (struct :`Roll` -90.0)) (`self.TreeSprite`) false (struct :`R` 1.0 :`G` 1.0 :`B` 1.0 :`A` 1.0)))))

(fn `UserConstructionScript`
  (`self.InitializeForestTiles`))