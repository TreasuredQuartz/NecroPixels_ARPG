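; BP_Fence is a spline-driven 2D fence actor that builds itself in the construction script, with no runtime logic.
; It steps along the spline by sprite length, adding grid-snapped, rotated FenceSprite instances to a Paper grouped sprite component.
; A single box is sized to the spline length, centered at its midpoint and aimed from the local origin toward the end, so it suits straight runs.
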(fn `UserConstructionScript`
  (bind _spritelength (`self.SpriteLength`))
  (bind _spritelength_2 (`self.SpriteLength`))
  (bind _returnvalue (/ (`SplineComponent.GetSplineLength` (`self.Spline`)) 2.0))
  (`|ExecutionSequence`
    (:`then_0`
      (`/Engine/EditorBlueprintResources/StandardMacros.IsValid` (`self.FenceSprite`)
        (:`Is Valid`
          (for _index (range (+ (`KismetMathLibrary.FTrunc` (/ (`SplineComponent.GetSplineLength` (`self.Spline`)) (`self.SpriteLength`))) 1))
            (bind (_returnvalue_x _returnvalue_y) (`KismetMathLibrary.BreakVector` (`SplineComponent.GetLocationAtDistanceAlongSpline` (`self.Spline`) (* _index (`self.SpriteLength`)) "Local")))
            (`PaperGroupedSpriteComponent.AddInstance` (`self.PaperGroupedSprite`) (`KismetMathLibrary.MakeTransform` (`KismetMathLibrary.MakeVector` (+ (* (`KismetMathLibrary.FTrunc` (/ _returnvalue_x _spritelength_2)) _spritelength) (/ (`self.SpriteLength`) 2.0)) (- (* (`KismetMathLibrary.FTrunc` (/ _returnvalue_y _spritelength_2)) _spritelength) (/ (`self.SpriteLength`) 2.0))) (struct :`Roll` -90.0)) (`self.FenceSprite`) false (struct :`R` 1.0 :`G` 1.0 :`B` 1.0 :`A` 1.0))))))
    (:`then_1`
      (`BoxComponent.SetBoxExtent` (`self.Box`) (`KismetMathLibrary.MakeVector` _returnvalue 16.0 32.0) false)
      (`SceneComponent.K2_SetRelativeLocation` (`self.Box`) (+ (`SplineComponent.GetLocationAtDistanceAlongSpline` (`self.Spline`) _returnvalue "Local") (0.0 0.0 32.0)) false false)
      (`SceneComponent.K2_SetRelativeRotation` (`self.Box`) (`KismetMathLibrary.FindLookAtRotation` (`KismetMathLibrary.MakeVector` 0.0) (`SplineComponent.GetLocationAtSplinePoint` (`self.Spline`) (`SplineComponent.GetNumberOfSplinePoints` (`self.Spline`)) "Local")) false false))))