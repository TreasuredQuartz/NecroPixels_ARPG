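; Red Nocturne character Blueprint that handles the character's reaction to taking damage.
; Its damage handler plays an on-hit animation override through the animation component's AnimInstance.
; An unconnected branch, which never runs, would award score by kill and damage type and record kills, headshots and score through GameState score and stat-tracker components.
; The construction script is empty.
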(fn `OnDamaged_0`
  (params (Player :type "PlayerState Object Reference") (DamageType :type "DamageType Object Reference"))
  (locals (ScoreManager :type "/Game/NecroPixelsContent/Components/ScoreManagerComponent Object Reference") (ScoreToAward :type Integer :default 10) (StatManager :type "/Game/NecroPixelsContent/Components/StatTrackerManagerComponent Object Reference"))
  (`PaperZDAnimInstance.K2_PlayAnimationOverride` (`PaperZDAnimationComponent.AnimInstance` (`self.AnimationComponent`)) (`self.OnHitAnimSequence_0`) "DefaultSlot" 1.0 0.0))

(fn `UserConstructionScript`)