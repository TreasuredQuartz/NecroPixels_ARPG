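; Skeleton melee swing attack actor, shown as a one-shot Paper2D flipbook animation.
; On BeginPlay it plays the flipbook without looping, then hides and destroys itself when playback finishes, so the animation sets the attack's lifetime.
; Actors that begin overlapping it are hit through HitActor if they are valid and pass ShouldHitActor.
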(event `self.ReceiveBeginPlay`
  (bind _paperflipbook (`self.PaperFlipbook`))
  (add `PaperFlipbookComponent.OnFinishedPlaying` (`self.PaperFlipbook`) (delegate `OnFinishedPlaying`))
  (`PaperFlipbookComponent.SetLooping` _paperflipbook false)
  (`PaperFlipbookComponent.Play` _paperflipbook))

(event `OnFinishedPlaying`
  (`self.SetActorHiddenInGame` true)
  (`self.K2_DestroyActor`))

(event `self.ReceiveActorBeginOverlap`
  (params (OtherActor :type "Actor Object Reference"))
  (`/Engine/EditorBlueprintResources/StandardMacros.IsValid` OtherActor
    (:`Is Valid`
      (bind _bshouldhitactor (`self.ShouldHitActor` OtherActor))
      (if _bshouldhitactor
        (`self.HitActor` OtherActor)))))

(fn `UserConstructionScript`
  (`parent.UserConstructionScript`))