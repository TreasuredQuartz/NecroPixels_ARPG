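; BP_Shadow is a non-playable shadow character whose sprite sinks and tips flat when it hides.
; Every tick the sprite yaws to face the player camera, with roll blended from upright to 90 degrees by HideTimeline progress.
; HideComponent's update event plays or reverses that timeline, which also lowers the sprite by up to the capsule's half-height.
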(event `self.ReceiveTick`
  (params (DeltaSeconds :type "Float (single-precision)"))
  (bind _hidetimeline (`self.HideTimeline`))
  (`SceneComponent.K2_SetWorldRotation` (`self.Sprite`) (`KismetMathLibrary.MakeRotator` (`KismetMathLibrary.Lerp` 0.0 90.0 (/ (`TimelineComponent.GetPlaybackPosition` _hidetimeline) (`TimelineComponent.GetTimelineLength` _hidetimeline))) 0.0 (+ (.yaw (`KismetMathLibrary.FindLookAtRotation` (`SceneComponent.K2_GetComponentLocation` (`self.Sprite`)) (`PlayerCameraManager.GetCameraLocation` (`GameplayStatics.GetPlayerCameraManager` 0)))) 90.0)) false false))

(event `self.HideComponent.OnHideUpdated`
  (bind _hidetimeline (`self.HideTimeline`))
  (if (`/Game/NecroPixelsContent/Components/Pawns/HideComponent.bIsHidiing` (`self.HideComponent`))
    (`Timeline|HideTimeline` :!label _label
      (:`Update`
        _)
      (:`Finished`
        _))
    (`SceneComponent.K2_SetRelativeLocation` (`self.Sprite`) (`KismetMathLibrary.MakeVector` 0.0 0.0 (`KismetMathLibrary.Lerp` 0.0 (- 0.0 (`CapsuleComponent.CapsuleHalfHeight` (`self.CapsuleComponent`))) (/ (`TimelineComponent.GetPlaybackPosition` _hidetimeline) (`TimelineComponent.GetTimelineLength` _hidetimeline)))) false false)
    (else
      (goto _label :!via `Reverse`))))

(fn `UserConstructionScript`)