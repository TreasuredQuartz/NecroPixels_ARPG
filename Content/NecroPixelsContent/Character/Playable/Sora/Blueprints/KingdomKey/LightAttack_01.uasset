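; Sora's first Kingdom Key light attack, a short-lived actor that plays a non-looping Paper2D flipbook and detects hits along a spline.
; Each tick, remaining lifespan over initial lifespan samples the spline, so the hitbox travels from spline end to start as the actor expires.
; A box multi-trace there, extended along the actor's forward axis, skips already impacted actors and calls HitActor on those passing ShouldImpactActor.
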(event `self.ReceiveTick`
  (params (DeltaSeconds :type "Float (single-precision)"))
  (bind _returnvalue (`self.GetActorForwardVector`))
  (bind _tracelength (`self.TraceLength`))
  (bind _spline (`self.Spline`))
  (bind _returnvalue_2 (/ (`self.GetLifeSpan`) (`self.InitialLifeSpan`)))
  (bind _returnvalue_3 (`SplineComponent.GetLocationAtTime` _spline _returnvalue_2 "World" false))
  (bind _outhits (`KismetSystemLibrary.BoxTraceMultiByProfile` (+ (* _returnvalue _tracelength -1) _returnvalue_3) (+ (* _returnvalue _tracelength) _returnvalue_3) (25.0 5.0 40.0) (`SplineComponent.GetRotationAtTime` _spline _returnvalue_2 "World" false) "None" false (`self.ImpactedActors`)))
  (for _array_element _outhits
    (bind (_bblockinghit _binitialoverlap _time _distance _location _impactpoint _normal _impactnormal _physmat _hitactor) (`GameplayStatics.BreakHitResult` _array_element))
    (if (`self.ShouldImpactActor` _hitactor)
      (`self.HitActor` _hitactor))))

(event `self.ReceiveBeginPlay`
  (bind _paperflipbook (`self.PaperFlipbook`))
  (`PaperFlipbookComponent.SetLooping` _paperflipbook false)
  (`PaperFlipbookComponent.Play` _paperflipbook))

(fn `UserConstructionScript`
  (`parent.UserConstructionScript`))