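; Attack state machine for Sora's Kingdom Key, switching between Idle and Light Attack while caching the owner's PaperZD animation and movement components.
; Idle enters Light Attack on attack trigger 1; its falling check currently leads to the same attack either way.
; Light Attack plays an override animation, spawns an attached attack actor, and uses the playback return as cooldown before returning to Idle.
; The combo continuation window is stubbed.
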(event `self.InitializeState_BP`
  (`|ExecutionSequence`
    (:`then_0`
      (bind _component (message `/Game/NecroPixelsContent/Interfaces/PaperZDAnimationInterface.GetPaperZDAnimComp` (`self.OwningActor`)))
      (set `self.AnimationComp` _component))
    (:`then_1`
      (bind _outmovementcomponent (message `/Game/NecroPixelsContent/Interfaces/MovementInterface.GetMovementComponent` (`self.OwningActor`)))
      (set `self.MoveComp` _outmovementcomponent))))

(event `self.EvaluateStateMachine_BP`
  (params (DeltaTime :type "Float (single-precision)"))
  (set `self.TimeInState` (+ DeltaTime (`self.TimeInState`)))
  (switch `/Game/NecroPixelsContent/Character/Default/Blueprints/Attacks/Enum_CharacterAttackState` (`self.AttackState`)
    (:`NewEnumerator3`
      (`self.IdleState`))
    (:`NewEnumerator0`
      (`self.LightAttack`))))

(event `SetAttackState`
  (params (AttackState :type "/Game/NecroPixelsContent/Character/Default/Blueprints/Attacks/Enum_CharacterAttackState Enum" :default "NewEnumerator3"))
  (set `self.AttackState` AttackState)
  (set `self.TimeInState` 0.0))

(fn `IdleState`
  (if (== (`self.TriggerAttackType`) 1)
    (if (`NavMovementComponent.IsFalling` (cast `CharacterMovementComponent` (`self.MoveComp`) :!pure true))
      (`self.SetAttackState` "NewEnumerator0")
      (else
        (`self.SetAttackState` "NewEnumerator0")))))

(fn `LightAttack`
  (locals (LocAttackOverhead :type "PaperZDAnimSequence Object Reference" :default "/Script/PaperZD.PaperZDAnimSequence_Flipbook'/Game/NecroPixelsContent/Character/Playable/Sora/Animations/ASeq_Sora_Attack_Overhead.ASeq_Sora_Attack_Overhead'") (LocContinueCombo :type "Float (double-precision)" :default 0.1))
  (bind _returnvalue (`self.GetOwner`))
  (bind (_returnvalue_location _returnvalue_rotation) (`KismetMathLibrary.BreakTransform` (`self.GetTransform` _returnvalue)))
  (if (<= (`self.Cooldown`) 0.0)
    (bind _animationlength (`PaperZDAnimInstance.K2_PlayAnimationOverride` (`PaperZDAnimationComponent.AnimInstance` (`self.AnimationComp`)) (`local.LocAttackOverhead`) "DefaultSlot" 1.0 0.0))
    (set `self.Cooldown` _animationlength)
    (bind _returnvalue_2 (`|SpawnActorFromClass` "/Game/NecroPixelsContent/Character/Playable/Sora/Blueprints/KingdomKey/LightAttack_01.LightAttack_01_C" (`KismetMathLibrary.MakeTransform` _returnvalue_location (`KismetMathLibrary.ComposeRotators` _returnvalue_rotation (`KismetMathLibrary.MakeRotator` 0.0)) (3.0 3.0 3.0)) "Undefined" "MultiplyWithRoot" (`self.GetOwner`) null))
    (`self.K2_AttachToActor` _returnvalue_2 _returnvalue "None" "KeepWorld" "KeepWorld" "KeepWorld" false)
    (elif (>= (`self.TimeInState`) (`self.Cooldown`))
      (set `self.Cooldown` 0.0)
      (`self.SetAttackState` "NewEnumerator3")
      (elif (>= (`self.TimeInState`) (`local.LocContinueCombo`))
        (if (== (`self.TriggerAttackType`) 1)
          _)))))

(fn `UserConstructionScript`)