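; KingdomKey is Sora's equippable Kingdom Key weapon Blueprint, which handles primary attack input.
; On equip, the EquippableComponent event initializes the AttackComponent's state with the weapon itself.
; The IA_AttackPrimary input feeds the AttackComponent as a binary attack input.
; Getter functions expose the owner's movement and PaperZD animation components, so the weapon works through its wielder's components.
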(event `EnhancedInput|/Game/NecroPixelsContent/Input/IA_AttackPrimary`
  (params (ActionValue :type Boolean) (ElapsedSeconds :type "Float (double-precision)") (TriggeredSeconds :type "Float (double-precision)") (InputAction :type "InputAction Object Reference" :default "/Game/NecroPixelsContent/Input/IA_AttackPrimary.IA_AttackPrimary"))
  (:`Triggered`
    (`/Game/NecroPixelsContent/Components/AttackComponent.AddAttackInput` (`self.AttackComponent`) (select `bool` ActionValue :`true` 1 :!type "Byte"))))

(event `self.EquippableComponent.OnEquipped`
  (`/Game/NecroPixelsContent/Components/AttackComponent.InitState` (`self.AttackComponent`) self))

(fn `GetMovementComponent`
  (returns (OutMovementComponent :type "MovementComponent Object Reference"))
  (return (`self.GetComponentByClass` (`self.GetOwner`) "/Script/Engine.MovementComponent")))

(fn `GetPaperZDAnimComp`
  (returns (Component :type "PaperZDAnimationComponent Object Reference"))
  (return (`self.GetComponentByClass` (`self.GetOwner`) "/Script/PaperZD.PaperZDAnimationComponent")))

(fn `UserConstructionScript`
  (`parent.UserConstructionScript`))