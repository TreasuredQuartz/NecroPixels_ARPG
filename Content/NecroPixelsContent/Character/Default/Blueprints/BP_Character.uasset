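; BP_Character is the default player-controllable character, with health, interaction and Paper animation components.
; On BeginPlay it adds its Enhanced Input mapping context, and IA_Move drives movement directly along world X and Y.
; Incoming damage goes to HealthComponent, whose health-zeroed event deactivates movement and interaction on death.
; Getters expose the health and animation components.
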(event `self.ReceiveBeginPlay`
  (`self.AddInputMappingContext`)
  (add `/Game/NecroPixelsContent/Components/Pawns/HealthComponent.OnHealthZeroed` (`self.HealthComponent`) (delegate `OnDeath`)))

(event `OnDeath`
  (`ActorComponent.Deactivate` (`self.CharacterMovement`))
  (`ActorComponent.Deactivate` (`self.InteractComponent`)))

(event `EnhancedInput|/Game/NecroPixelsContent/Input/IA_Move`
  (params (ActionValue :type "Vector2D Structure") (ElapsedSeconds :type "Float (double-precision)") (TriggeredSeconds :type "Float (double-precision)") (InputAction :type "InputAction Object Reference" :default "/Game/NecroPixelsContent/Input/IA_Move.IA_Move"))
  (bind (_x _y) (`KismetMathLibrary.BreakVector2D` ActionValue))
  (:`Triggered`
    (`self.AddMovementInput` (`KismetMathLibrary.MakeVector` _x _y))))

(event `self.ReceiveAnyDamage`
  (params (Damage :type "Float (single-precision)") (DamageType :type "DamageType Object Reference") (InstigatedBy :type "Controller Object Reference") (DamageCauser :type "Actor Object Reference"))
  (`/Game/NecroPixelsContent/Components/Pawns/HealthComponent.DealDamage` (`self.HealthComponent`) Damage))

(fn `AddInputMappingContext`
  (bind _asplayer_controller (cast `PlayerController` (`self.GetController`)))
  (bind _returnvalue (pcsubsystem `EnhancedInputLocalPlayerSubsystem` _asplayer_controller))
  (`/Engine/EditorBlueprintResources/StandardMacros.IsValid` _returnvalue
    (:`Is Valid`
      (`EnhancedInputSubsystemInterface.AddMappingContext` _returnvalue "/Game/NecroPixelsContent/Input/MappingContext.MappingContext" 0 (struct)))))

(fn `GetHealthComponent`
  (returns (OutHealthComponent :type "/Game/NecroPixelsContent/Components/Pawns/HealthComponent Object Reference"))
  (return (`self.HealthComponent`)))

(fn `GetPaperAnimationComponent`
  (returns (OutPaperAnimationComponent :type "/Game/NecroPixelsContent/Components/Pawns/PaperAnimationComponent Object Reference"))
  (return (`self.PaperAnimationComponent`)))

(fn `UserConstructionScript`)