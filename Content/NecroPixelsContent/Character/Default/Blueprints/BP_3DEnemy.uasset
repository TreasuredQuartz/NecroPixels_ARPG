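; BP_3DEnemy is an enemy character with a sprite, health and a PaperZD-style animation component.
; On spawn it stops the sprite looping and waits briefly before activating movement and looped playback.
; Damage feeds the HealthComponent and, when the instigator has a valid PlayerState, plays a hit animation override.
; At zero health it disables movement and collision, then expires after a short lifespan.
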(event `self.ReceiveBeginPlay`
  (bind _sprite (`self.Sprite`))
  (`PaperFlipbookComponent.SetLooping` (`self.Sprite`) false)
  (`KismetSystemLibrary.Delay` 0.8)
  (`ActorComponent.Activate` (`self.CharacterMovement`) false)
  (`PaperFlipbookComponent.SetLooping` _sprite true)
  (`PaperFlipbookComponent.Play` _sprite))

(event `self.HealthComponent.OnHealthZeroed`
  (`ActorComponent.Deactivate` (`self.CharacterMovement`))
  (`self.SetActorEnableCollision` false)
  (`self.SetLifeSpan` 1.0))

(event `self.ReceiveAnyDamage`
  (params (Damage :type "Float (single-precision)") (DamageType :type "DamageType Object Reference") (InstigatedBy :type "Controller Object Reference") (DamageCauser :type "Actor Object Reference"))
  (bind _playerstate (`Controller.PlayerState` InstigatedBy))
  (`/Game/NecroPixelsContent/Components/HealthComponent.DealDamage` (`self.HealthComponent`) Damage)
  (`/Engine/EditorBlueprintResources/StandardMacros.IsValid` _playerstate
    (:`Is Valid`
      (`self.OnDamaged` _playerstate DamageType))))

(fn `OnDamaged`
  (params (Player :type "PlayerState Object Reference") (DamageType :type "DamageType Object Reference"))
  (`PaperZDAnimInstance.K2_PlayAnimationOverride` (`PaperZDAnimationComponent.AnimInstance` (`self.AnimationComponent`)) (`self.OnHitAnimSequence`) "DefaultSlot" 1.0 0.0))

(fn `UserConstructionScript`
  (`parent.UserConstructionScript`))