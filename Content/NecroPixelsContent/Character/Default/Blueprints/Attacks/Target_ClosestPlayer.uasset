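; Targeting actor for Necro Pixels characters that attaches to its owner and writes the assigned target to the owner's AI blackboard.
; Start and stop targeting only call the parent class.
; Helpers validate targets by health and opposing team and sample a random sphere-trace hit, but the retargeting logic using them is disconnected.
; Despite the ClosestPlayer name, no closest-player search exists in this graph.
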(event `self.ReceiveBeginPlay`
  (`self.K2_AttachToActor` (`self.GetOwner`) "None" "KeepRelative" "KeepRelative" "KeepRelative"))

(event `self.ReceiveTick`
  (params (DeltaSeconds :type "Float (single-precision)")))

(event `self.StartTargeting`
  (`parent.StartTargeting`))

(event `self.StopTargeting`
  (`parent.StopTargeting`))

(event `SetTargetActor`
  (params (TargetActor :type "Actor Object Reference"))
  (bind _returnvalue (`AIBlueprintHelperLibrary.GetBlackboard` (`AIBlueprintHelperLibrary.GetAIController` (`self.GetOwner`))))
  (set `self.TargetActor` TargetActor)
  (`/Engine/EditorBlueprintResources/StandardMacros.IsValid` _returnvalue
    (:`Is Valid`
      (`BlackboardComponent.SetValueAsObject` _returnvalue (`self.TargetActorKeyName`) (`self.TargetActor`)))))

(fn `FindRandomTargetWithinRadius`
  (params (Radius :type "Float (single-precision)"))
  (returns (NewTargetActor :type "Actor Object Reference"))
  (locals (PotentialTarget :type "Actor Object Reference"))
  (bind _returnvalue (`self.K2_GetActorLocation` self))
  (bind (_outhits _returnvalue_2) (`KismetSystemLibrary.SphereTraceMultiByProfile` _returnvalue _returnvalue Radius "Pawn" false (`|MakeArray` self (`self.GetOwner`) :!type "Actor Object Reference")))
  (if _returnvalue_2
    (bind _output_get (set `local.PotentialTarget` (`.HitActor` (`GameplayStatics.BreakHitResult` (`|GetArrayItem` _outhits (`KismetMathLibrary.RandomIntegerInRange` 0 (- (`KismetArrayLibrary.Array_Length` _outhits) 1)))))))
    (`/Engine/EditorBlueprintResources/StandardMacros.IsValid` _output_get
      (:`Is Valid`
        (bind _bisvalid (`self.IsActorValidTarget` (`local.PotentialTarget`)))
        (if (not _bisvalid)
          (set `local.PotentialTarget` null))))
    (else
      (return (`local.PotentialTarget`)))))

(fn `IsActorValidTarget`
  (params (Actor :type "Actor Object Reference"))
  (returns (bIsValid :type Boolean))
  (locals (Target :type "Actor Object Reference"))
  (bind _returnvalue (`self.GetComponentByClass` (`local.Target`) "/Game/NecroPixelsContent/Components/TeamComponent.TeamComponent_C"))
  (bind _returnvalue_2 (`self.GetComponentByClass` (`self.GetOwner`) "/Game/NecroPixelsContent/Components/TeamComponent.TeamComponent_C"))
  (bind _output_get (set `local.Target` Actor))
  (`/Engine/EditorBlueprintResources/StandardMacros.IsValid` _output_get
    (:`Is Valid`
      ;[1 1 1] Health Component
      (bind _outhealthcomponent (message `/Game/NecroPixelsContent/Interfaces/HealthSystemInterface.GetHealthComponent` (`local.Target`)))
      (`/Engine/EditorBlueprintResources/StandardMacros.IsValid` _outhealthcomponent
        (:`Is Valid`
          (if (not (`/Game/NecroPixelsContent/Components/HealthComponent.bIsHealthZero` _outhealthcomponent))
            ;[1 1 1] Team Componment
            (`/Engine/EditorBlueprintResources/StandardMacros.IsValid` _returnvalue_2
              (:`Is Valid`
                (`/Engine/EditorBlueprintResources/StandardMacros.IsValid` _returnvalue
                  (:`Is Valid`
                    (if (!= (`/Game/NecroPixelsContent/Components/TeamComponent.TeamID` _returnvalue) (`/Game/NecroPixelsContent/Components/TeamComponent.TeamID` _returnvalue_2))
                      (return true)
                      (else
                        _)))
                  (:`Is Not Valid`
                    _)))
              (:`Is Not Valid`
                _))))
        (:`Is Not Valid`
          _)))
    (:`Is Not Valid`
      _))
  (return false))

(fn `UserConstructionScript`
  (`parent.UserConstructionScript`))