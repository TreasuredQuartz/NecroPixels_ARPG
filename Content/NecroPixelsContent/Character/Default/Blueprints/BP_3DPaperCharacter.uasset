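; Paper2D character for a 3D world whose sprite billboards toward the camera and mirrors horizontally to match its movement direction.
; Each tick it yaws the sprite at the player camera, then MirrorSprite flips its X scale.
; While moving, the flip follows input X from Input2DMovementComponent and the last horizontal velocity direction is stored.
; When idle, that stored direction is compared with a camera-relative right vector to choose the flip.
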(event `self.ReceiveTick`
  (params (DeltaSeconds :type "Float (single-precision)"))
  (`SceneComponent.K2_SetWorldRotation` (`self.Sprite`) (`KismetMathLibrary.MakeRotator` 0.0 0.0 (+ (.yaw (`KismetMathLibrary.FindLookAtRotation` (`SceneComponent.K2_GetComponentLocation` (`self.Sprite`)) (`PlayerCameraManager.GetCameraLocation` (`GameplayStatics.GetPlayerCameraManager` 0)))) 90.0)) false false)
  (`self.MirrorSprite`))

(fn `MirrorSprite`
  (bind _returnvalue (`KismetMathLibrary.Conv_VectorToVector2D` (`self.GetVelocity`)))
  (if (> (`KismetMathLibrary.VSize` (`self.GetVelocity`)) 0.0)
    (`SceneComponent.SetRelativeScale3D` (`self.Sprite`) (`KismetMathLibrary.MakeVector` (`KismetMathLibrary.SelectFloat` -3.0 3.0 (> (`KismetMathLibrary.BreakVector2D` (`/Game/NecroPixelsContent/Components/Input_2DMovementComponent.InputMoveDirection` (`self.Input_2DMovementComponent`))) 0.0)) 3.0 3.0))
    (if (> (`KismetMathLibrary.VSize2D` _returnvalue) 0.0)
      (set `self.LastVelocity2D` (`KismetMathLibrary.Normal2D` _returnvalue)))
    (elif (> (`KismetMathLibrary.DotProduct2D` (`KismetMathLibrary.Normal2D` (`KismetMathLibrary.Conv_VectorToVector2D` (`KismetMathLibrary.GetRightVector` (`KismetMathLibrary.FindLookAtRotation` (`self.K2_GetActorLocation`) (`PlayerCameraManager.GetCameraLocation` (`GameplayStatics.GetPlayerCameraManager` 0)))))) (`self.LastVelocity2D`)) 0.0)
      (`SceneComponent.SetRelativeScale3D` (`self.Sprite`) (-3.0 3.0 3.0))
      (else
        (`SceneComponent.SetRelativeScale3D` (`self.Sprite`) (3.0 3.0 3.0))))))

(fn `UserConstructionScript`)