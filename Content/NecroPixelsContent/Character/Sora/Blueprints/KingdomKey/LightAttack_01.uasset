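; Short-lived 2D attack actor for the first Kingdom Key light attack of the Sora character.
; It plays its Paper2D flipbook once on BeginPlay, then hides and destroys itself when playback finishes.
; Overlapping actors that pass ShouldImpactActor are passed to HitActor.
; Tick resets the actor's world rotation to zero every frame.
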(event `self.ReceiveTick`
  (params (DeltaSeconds :type "Float (single-precision)"))
  (`self.K2_SetActorRotation` (struct)))

(event `self.ReceiveBeginPlay`
  (bind _paperflipbook (`self.PaperFlipbook`))
  (add `PaperFlipbookComponent.OnFinishedPlaying` (`self.PaperFlipbook`) (delegate `OnFinishedPlaying`))
  (`PaperFlipbookComponent.SetLooping` _paperflipbook false)
  (`PaperFlipbookComponent.Play` _paperflipbook))

(event `OnFinishedPlaying`
  (`self.SetActorHiddenInGame` true)
  (`self.K2_DestroyActor`))

(event `self.ReceiveActorBeginOverlap`
  (params (OtherActor :type "Actor Object Reference"))
  (if (`self.ShouldImpactActor` OtherActor)
    (`self.HitActor` OtherActor)))

(fn `UserConstructionScript`
  (`parent.UserConstructionScript`))