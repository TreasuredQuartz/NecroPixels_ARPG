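; BP_3DPaperCharacter is a player-controlled Paper2D sprite character that handles Enhanced Input setup, jumping and landing.
; A 2D movement component's updates flip the sprite horizontally by input direction, except during ledge grabs.
; Jump input passes through an input buffer and ledge-grab check, then sets a wants-to-jump flag and jumps after a short delay.
; Landing briefly disables player input.
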(event `self.ReceiveBeginPlay`
  (bind _asplayer_controller (cast `PlayerController` (`self.GetController`)))
  (bind _returnvalue (pcsubsystem `EnhancedInputLocalPlayerSubsystem` _asplayer_controller))
  (`/Engine/EditorBlueprintResources/StandardMacros.IsValid` _returnvalue
    (:`Is Valid`
      (`EnhancedInputSubsystemInterface.AddMappingContext` _returnvalue "/Game/NecroPixelsContent/Input/MappingContext.MappingContext" 0 (struct)))))

(event `self.Input_2DMovementComponent.OnMovementUpdated`
  (bind _x (`KismetMathLibrary.BreakVector2D` (`/Game/NecroPixelsContent/Components/Input_2DMovementComponent.InputDirection` (`self.Input_2DMovementComponent`))))
  (if (`/Game/NecroPixelsContent/Components/LedgeGrabComponent.IsLedgeGrabbing` (`self.LedgeGrabComponent`))
    _
    (elif (!= _x 0.0)
      (`SceneComponent.SetRelativeScale3D` (`self.Sprite`) (`KismetMathLibrary.MakeVector` (`KismetMathLibrary.SelectFloat` -3.0 3.0 (> _x 0.0)) 3.0 3.0)))))

(event `StartJump`
  (set `self.bWantsToJump` true)
  (`KismetSystemLibrary.Delay` 0.15)
  (`self.Jump`)
  (set `self.bWantsToJump` false))

(event `EnhancedInput|/Game/NecroPixelsContent/Input/IA_Jump`
  (params (ActionValue :type Boolean) (ElapsedSeconds :type "Float (double-precision)") (TriggeredSeconds :type "Float (double-precision)") (InputAction :type "InputAction Object Reference" :default "/Game/NecroPixelsContent/Input/IA_Jump.IA_Jump"))
  (:`Triggered`
    (bind _canbufferinput (`/Game/NecroPixelsContent/Components/InputBufferComponent.PushInputOntoBuffer` (`self.InputBufferComponent`) InputAction))
    (if _canbufferinput
      _
      (elif (`/Game/NecroPixelsContent/Components/LedgeGrabComponent.IsLedgeGrabbing` (`self.LedgeGrabComponent`))
        _
        (elif ActionValue
          (`self.StartJump`)
          (else
            (`self.StopJumping`)
            (set `self.bWantsToJump` false)))))))

(event `self.OnLanded`
  (params (Hit :type "HitResult Structure (by ref)"))
  (bind _asplayer_controller (cast `PlayerController` (`self.GetController`) :!pure true))
  (`self.DisableInput` _asplayer_controller)
  (`KismetSystemLibrary.Delay` 0.2)
  (`self.EnableInput` _asplayer_controller))

(event `self.OnJumped`)

(fn `UserConstructionScript`)