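; Player-controlled paper sprite character for a 3D world, with movement and jumping through Enhanced Input.
; BeginPlay adds the mapping context, and the move action feeds its 2D value straight into world X/Y movement.
; Facing mirrors the sprite by flipping its X scale on horizontal input, keeping the last facing otherwise.
; Jump follows the action value, and landing briefly disables input as a recovery pause.
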(event `self.ReceiveBeginPlay`
  (bind _asplayer_controller (cast `PlayerController` (`self.GetController`)))
  (bind _returnvalue (pcsubsystem `EnhancedInputLocalPlayerSubsystem` _asplayer_controller))
  (`/Engine/EditorBlueprintResources/StandardMacros.IsValid` _returnvalue
    (:`Is Valid`
      (`EnhancedInputSubsystemInterface.AddMappingContext` _returnvalue "/Game/NecroPixelsContent/Input/MappingContext.MappingContext" 0 (struct)))))

(event `EnhancedInput|/Game/NecroPixelsContent/Input/IA_Move`
  (params (ActionValue :type "Vector2D Structure") (ElapsedSeconds :type "Float (double-precision)") (TriggeredSeconds :type "Float (double-precision)") (InputAction :type "InputAction Object Reference" :default "/Game/NecroPixelsContent/Input/IA_Move.IA_Move"))
  (bind (_inputdirection_x _inputdirection_y) (`KismetMathLibrary.BreakVector2D` (`self.InputDirection`)))
  (:`Triggered`
    (set `self.InputDirection` ActionValue)
    (`self.AddMovementInput` (`KismetMathLibrary.MakeVector` _inputdirection_x _inputdirection_y))
    (`self.UpdateFacing`)))

(event `UpdateFacing`
  (bind _x (`KismetMathLibrary.BreakVector2D` (`self.InputDirection`)))
  (if (!= _x 0.0)
    (`SceneComponent.SetRelativeScale3D` (`self.Sprite`) (`KismetMathLibrary.MakeVector` (`KismetMathLibrary.SelectFloat` -3.0 3.0 (> _x 0.0)) 3.0 3.0))))

(event `EnhancedInput|/Game/NecroPixelsContent/Input/IA_Jump`
  (params (ActionValue :type Boolean) (ElapsedSeconds :type "Float (double-precision)") (TriggeredSeconds :type "Float (double-precision)") (InputAction :type "InputAction Object Reference" :default "/Game/NecroPixelsContent/Input/IA_Jump.IA_Jump"))
  (:`Triggered`
    (if ActionValue
      (`self.Jump`)
      (else
        (`self.StopJumping`)))))

(event `self.OnLanded`
  (params (Hit :type "HitResult Structure (by ref)"))
  (bind _asplayer_controller (cast `PlayerController` (`self.GetController`) :!pure true))
  (`self.DisableInput` _asplayer_controller)
  (`KismetSystemLibrary.Delay` 0.2)
  (`self.EnableInput` _asplayer_controller))

(fn `UserConstructionScript`)