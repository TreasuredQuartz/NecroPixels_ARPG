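; AI controller for skeleton enemies that runs the BT_Horde behavior tree to go after players.
; On possess it picks the closest living player character, writes it to the blackboard target key, and clears the key when none remain.
; It binds to the target's HealthComponent zero-health event, apparently to retarget when that player dies.
; It also binds to its own pawn's zero-health event to stop the brain logic on death.
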(event `self.ReceiveBeginPlay`
  (`self.RunBehaviorTree` "/Game/NecroPixelsContent/AI/BT_Horde.BT_Horde"))

(event `OnTargetDied`
  (`self.FindNewTargetActor`))

(event `self.ReceivePossess`
  (params (PossessedPawn :type "Pawn Object Reference"))
  (bind _returnvalue (`self.K2_GetPawn`))
  (bind _returnvalue_2 (`self.GetComponentByClass` _returnvalue "/Game/NecroPixelsContent/Components/HealthComponent.HealthComponent_C"))
  (`/Engine/EditorBlueprintResources/StandardMacros.IsValid` _returnvalue
    (:`Is Valid`
      (`|ExecutionSequence`
        (:`then_0`
          (`self.FindNewTargetActor`)
          (`/Engine/EditorBlueprintResources/StandardMacros.IsValid` _returnvalue_2
            (:`Is Valid`
              (add `/Game/NecroPixelsContent/Components/HealthComponent.OnHealthZeroed` _returnvalue_2 (delegate `OnDeath`)))))))))

(event `OnDeath`
  (`BrainComponent.StopLogic` (`self.BrainComponent`) "Death"))

(fn `FindNewTargetActor`
  (locals (PotentialTargets :type "Array of Character Object Reference") (ClosestTarget :type "Character Object Reference") (ClosestDistance :type "Float (double-precision)"))
  (bind _potentialtargets (`local.PotentialTargets`))
  (`/Engine/EditorBlueprintResources/StandardMacros.IsValid` (`self.K2_GetPawn`)
    (:`Is Valid`
      (bind _returnvalue (`GameModeBase.GetNumPlayers` (`GameplayStatics.GetGameMode`)))
      (for _index (range _returnvalue)
        (bind _returnvalue_2 (`GameplayStatics.GetPlayerCharacter` _index))
        (`/Engine/EditorBlueprintResources/StandardMacros.IsValid` _returnvalue_2
          (:`Is Valid`
            (bind _returnvalue_3 (`self.GetComponentByClass` _returnvalue_2 "/Game/NecroPixelsContent/Components/HealthComponent.HealthComponent_C"))
            (`/Engine/EditorBlueprintResources/StandardMacros.IsValid` _returnvalue_3
              (:`Is Valid`
                (if (not (`/Game/NecroPixelsContent/Components/HealthComponent.bIsHealthZero` _returnvalue_3))
                  (`KismetArrayLibrary.Array_Add` (`local.PotentialTargets`) _returnvalue_2)))))))
      (if (`KismetArrayLibrary.Array_IsNotEmpty` _potentialtargets)
        (for _array_element _potentialtargets
          (`/Engine/EditorBlueprintResources/StandardMacros.IsValid` (`local.ClosestTarget`)
            (:`Is Valid`
              (bind _returnvalue_4 (`KismetMathLibrary.Vector_Distance` (`self.K2_GetActorLocation` _array_element) (`self.K2_GetActorLocation` (`self.K2_GetPawn`))))
              (if (< _returnvalue_4 (`local.ClosestDistance`))
                (set `local.ClosestDistance` _returnvalue_4)
                (set `local.ClosestTarget` _array_element)))
            (:`Is Not Valid`
              (bind _output_get (set `local.ClosestTarget` _array_element))
              (set `local.ClosestDistance` (`KismetMathLibrary.Vector_Distance` (`self.K2_GetActorLocation` _output_get) (`self.K2_GetActorLocation` (`self.K2_GetPawn`)))))))
        (`self.SetTargetActor` (`local.ClosestTarget`))
        (else
          (`self.SetTargetActor` null))))))

(fn `SetTargetActor`
  (params (NewTargetActor :type "Actor Object Reference"))
  (bind _returnvalue (`self.GetComponentByClass` (`local.NewTargetActor`) "/Game/NecroPixelsContent/Components/HealthComponent.HealthComponent_C"))
  (`BlackboardComponent.SetValueAsObject` (`AIBlueprintHelperLibrary.GetBlackboard` null) (`self.TargetKey`) NewTargetActor)
  (`/Engine/EditorBlueprintResources/StandardMacros.IsValid` (`local.NewTargetActor`)
    (:`Is Valid`
      (`/Engine/EditorBlueprintResources/StandardMacros.IsValid` _returnvalue
        (:`Is Valid`
          (add `/Game/NecroPixelsContent/Components/HealthComponent.OnHealthZeroed` _returnvalue (`|CreateDelegate` :!event `OnTargetDied`)))))))

(fn `UserConstructionScript`)