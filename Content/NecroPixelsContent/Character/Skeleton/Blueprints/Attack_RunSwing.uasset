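; Short-lived hitbox actor for the skeleton's running swing attack, which destroys itself after one second.
; On overlap it skips its owner, same-team actors, and opposing-team actors without health or already dead.
; If either side lacks a TeamComponent, the team and health checks are both bypassed.
; Each actor takes blunt-force damage only once, and successful damage is reported to the owner's AttackComponent.
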(event `self.ReceiveBeginPlay`
  (`self.SetLifeSpan` 1.0))

(event `self.ReceiveActorBeginOverlap`
  (params (OtherActor :type "Actor Object Reference"))
  (bind _returnvalue (`self.GetComponentByClass` OtherActor "/Game/NecroPixelsContent/Components/TeamComponent.TeamComponent_C"))
  (bind _returnvalue_2 (`self.GetOwner`))
  (bind _returnvalue_3 (`self.GetComponentByClass` OtherActor "/Game/NecroPixelsContent/Components/HealthComponent.HealthComponent_C"))
  (bind _returnvalue_4 (`self.GetComponentByClass` (`self.GetOwner`) "/Game/NecroPixelsContent/Components/TeamComponent.TeamComponent_C"))
  (`/Engine/EditorBlueprintResources/StandardMacros.IsValid` OtherActor
    (:`Is Valid`
      (`/Engine/EditorBlueprintResources/StandardMacros.IsValid` _returnvalue_2
        (:`Is Valid`
          (if (!= _returnvalue_2 OtherActor)
            (`/Engine/EditorBlueprintResources/StandardMacros.IsValid` _returnvalue_4
              (:`Is Valid`
                (`/Engine/EditorBlueprintResources/StandardMacros.IsValid` _returnvalue
                  (:`Is Valid`
                    (if (!= (`/Game/NecroPixelsContent/Components/TeamComponent.TeamID` _returnvalue_4) (`/Game/NecroPixelsContent/Components/TeamComponent.TeamID` _returnvalue))
                      (`/Engine/EditorBlueprintResources/StandardMacros.IsValid` _returnvalue_3 ; Only Attack things that have health...
                        (:`Is Valid`
                          (if (not (`/Game/NecroPixelsContent/Components/HealthComponent.bIsHealthZero` _returnvalue_3))
                            (if (not (`KismetArrayLibrary.Array_Contains` (`self.OverlappedActors`) OtherActor)) :!label _label
                              (`KismetArrayLibrary.Array_Add` (`self.OverlappedActors`) OtherActor)
                              (bind _returnvalue_5 (`GameplayStatics.ApplyDamage` OtherActor 50.0 (`self.GetInstigatorController`) self "/Game/NecroPixelsContent/DamageTypes/DmgType_BluntForce.DmgType_BluntForce_C"))
                              (if (> _returnvalue_5 0.0)
                                (`/Game/NecroPixelsContent/Components/AttackComponent.AttackedActor` (`self.GetComponentByClass` (`self.GetOwner`) "/Game/NecroPixelsContent/Components/AttackComponent.AttackComponent_C") OtherActor))))))))
                  (:`Is Not Valid`
                    (goto _label))))
              (:`Is Not Valid`
                (goto _label)))))))))

(fn `UserConstructionScript`
  (`parent.UserConstructionScript`))