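; Attack state machine for the 2D skeleton character, choosing and running its light and heavy melee attacks.
; When triggered from Idle, owner speed selects a light attack at shambling pace or a heavy one otherwise, re-evaluating immediately.
; Light attack locks movement through Anticipation, Action and Recovery; heavy attack fires on entry.
; Both play flipbook montages, spawn attached attack actors, and clear IsAttacking after a shared cooldown.
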(event `self.InitializeState_BP`
  (set `self.AttackComponent` (`self.GetComponentByClass` (`self.OwningActor`) "/Game/NecroPixelsContent/Components/AttackComponent.AttackComponent_C")))

(event `self.EvaluateStateMachine_BP`
  (params (DeltaTime :type "Float (single-precision)"))
  (set `self.TimeInState` (+ DeltaTime (`self.TimeInState`)))
  (switch `/Game/NecroPixelsContent/Character/Default/Blueprints/Attacks/Enum_CharacterAttackState` (`self.CharacterState`)
    (:`NewEnumerator3`
      (`self.IdleState`))
    (:`NewEnumerator0`
      (`self.LightAttackState`))
    (:`NewEnumerator1`
      (`self.HeavyAttackState`))))

(fn `CanAttack`)

(fn `HeavyAttackState`
  (locals (AttackStateCooldown :type "Float (double-precision)" :default 1.0) (HeavyAttackClass :type "/Game/NecroPixelsContent/AttackStateMachineGraph/BP_AttackInstance Class Reference" :default "/Script/Engine.BlueprintGeneratedClass'/Game/NecroPixelsContent/Character/Skeleton/Blueprints/Attack_RunSwing.Attack_RunSwing_C'") (HeavyAttackFlipbook :type "PaperFlipbook Object Reference" :default "/Script/Paper2D.PaperFlipbook'/Game/NecroPixelsContent/Character/Skeleton/Flipbooks/Flipbook_Skeleton_Attack.Flipbook_Skeleton_Attack'"))
  (bind _returnvalue (`self.GetOwner`))
  (bind _returnvalue_2 (`self.GetOwner`))
  (bind _returnvalue_3 (`self.GetOwner`))
  (bind (_returnvalue_location _returnvalue_rotation _returnvalue_scale) (`KismetMathLibrary.BreakTransform` (`SceneComponent.K2_GetComponentToWorld` (`self.GetComponentByClass` _returnvalue_2 "/Script/Paper2D.PaperFlipbookComponent"))))
  (if (== (`self.TimeInState`) 0.0)
    (`/Game/NecroPixelsContent/Components/PaperAnimationComponent.PlayMontage` (`self.GetComponentByClass` _returnvalue_2 "/Game/NecroPixelsContent/Components/PaperAnimationComponent.PaperAnimationComponent_C") (`local.HeavyAttackFlipbook`))
    (bind _returnvalue_4 (`|SpawnActorFromClass` (`local.HeavyAttackClass`) (`KismetMathLibrary.MakeTransform` _returnvalue_location _returnvalue_rotation _returnvalue_scale) "AlwaysSpawn" "MultiplyWithRoot" _returnvalue_3 (cast `Pawn` _returnvalue_3 :!pure true)))
    (`self.K2_AttachToActor` _returnvalue_4 (`self.GetOwner`) "None" "KeepWorld" "KeepWorld" "KeepWorld" true)
    (elif (>= (`self.TimeInState`) (`local.AttackStateCooldown`))
      (`/Engine/EditorBlueprintResources/StandardMacros.IsValid` _returnvalue
        (:`Is Valid`
          (bind _asbp_skeleton (cast `/Game/NecroPixelsContent/Character/Skeleton/Blueprints/BP_Skeleton` _returnvalue))
          (set `/Game/NecroPixelsContent/Character/Skeleton/Blueprints/BP_Skeleton.bIsAttacking` false _asbp_skeleton)
          (set `self.bIsAttacking` false)
          (set `self.CharacterState` "NewEnumerator3")
          (set `self.TimeInState` 0.0))))))

(fn `IdleState`
  (if (!= (`self.TriggerAttackType`) 0)
    (`self.ResetAttack`)
    (if (`self.IsShambling`)
      (set `self.CharacterState` "NewEnumerator0")
      (set `self.TimeInState` 0.0)
      (`self.EvaluateStateMachine` 0.0)
      (else
        (if (`self.IsSprinting`)
          _
          (else
            _))
        (set `self.CharacterState` "NewEnumerator1")
        (set `self.TimeInState` 0.0)
        (`self.EvaluateStateMachine` 0.0)))))

(fn `IsShambling`
  (returns (ReturnValue :type Boolean))
  (return (<= (`KismetMathLibrary.VSize` (`self.GetVelocity` (`self.GetOwner`))) 75.0)))

(fn `IsSprinting`
  (returns (ReturnValue :type Boolean))
  (return (> (`KismetMathLibrary.VSize` (`self.GetVelocity` (`self.GetOwner`))) 150.0)))

(fn `LightAttackState`
  (locals (AttackStateCooldown :type "Float (double-precision)" :default 1.0) (LightAttackClass :type "/Game/NecroPixelsContent/AttackStateMachineGraph/BP_AttackInstance Class Reference" :default "/Script/Engine.BlueprintGeneratedClass'/Game/NecroPixelsContent/Character/Skeleton/Blueprints/Attack_ShambleSwing.Attack_ShambleSwing_C'") (LightAttack_Flipbook :type "PaperFlipbook Object Reference" :default "/Script/Paper2D.PaperFlipbook'/Game/NecroPixelsContent/Character/Skeleton/Flipbooks/Flipbook_Skele_ShambleAttack.Flipbook_Skele_ShambleAttack'") (LightAttack_AnticipationTime :type "Float (double-precision)" :default 0.02))
  (bind _returnvalue (`self.GetOwner`))
  (bind _returnvalue_2 (`self.GetOwner`))
  (bind _returnvalue_3 (`self.GetOwner`))
  (bind _returnvalue_4 (`self.GetComponentByClass` (`self.GetOwner`) "/Script/Engine.CharacterMovementComponent"))
  (bind (_returnvalue_location _returnvalue_rotation _returnvalue_scale) (`KismetMathLibrary.BreakTransform` (`SceneComponent.K2_GetComponentToWorld` (`self.GetComponentByClass` _returnvalue_3 "/Script/Paper2D.PaperFlipbookComponent"))))
  (switch `/Game/NecroPixelsContent/Character/Default/Blueprints/Attacks/Enum_SubAttackState` (`self.AttackState`)
    (:`NewEnumerator0`
      (`CharacterMovementComponent.DisableMovement` _returnvalue_4)
      (`MovementComponent.StopMovementImmediately` _returnvalue_4)
      (set `self.AttackState` "NewEnumerator1"))
    (:`NewEnumerator1`
      (if (>= (`self.TimeInState`) (`local.LightAttack_AnticipationTime`))
        (set `self.AttackState` "NewEnumerator2")))
    (:`NewEnumerator2`
      (`/Game/NecroPixelsContent/Components/PaperAnimationComponent.PlayMontage` (`self.GetComponentByClass` _returnvalue_3 "/Game/NecroPixelsContent/Components/PaperAnimationComponent.PaperAnimationComponent_C") (`local.LightAttack_Flipbook`))
      (bind _returnvalue_5 (`|SpawnActorFromClass` (`local.LightAttackClass`) (`KismetMathLibrary.MakeTransform` (+ (* (`KismetMathLibrary.GetForwardVector` _returnvalue_rotation) (5.0 0.0 0.0)) _returnvalue_location) _returnvalue_rotation _returnvalue_scale) "AlwaysSpawn" "MultiplyWithRoot" _returnvalue_2 (cast `Pawn` _returnvalue_2 :!pure true)))
      (`self.K2_AttachToActor` _returnvalue_5 (`self.GetOwner`) "None" "KeepWorld" "KeepWorld" "KeepWorld" true)
      (set `self.AttackState` "NewEnumerator3"))
    (:`NewEnumerator3`
      (if (>= (`self.TimeInState`) (`local.AttackStateCooldown`))
        (`/Engine/EditorBlueprintResources/StandardMacros.IsValid` _returnvalue
          (:`Is Valid`
            (bind _asbp_skeleton (cast `/Game/NecroPixelsContent/Character/Skeleton/Blueprints/BP_Skeleton` _returnvalue))
            (set `/Game/NecroPixelsContent/Character/Skeleton/Blueprints/BP_Skeleton.bIsAttacking` false _asbp_skeleton)
            (set `self.bIsAttacking` false)
            (set `self.CharacterState` "NewEnumerator3")
            (set `self.TimeInState` 0.0)
            (set `self.AttackState` "NewEnumerator0")
            (`CharacterMovementComponent.SetMovementMode` (`self.GetComponentByClass` (`self.GetOwner`) "/Script/Engine.CharacterMovementComponent") "MOVE_Walking" 0)))))))

(fn `UserConstructionScript`
  (`parent.UserConstructionScript`))