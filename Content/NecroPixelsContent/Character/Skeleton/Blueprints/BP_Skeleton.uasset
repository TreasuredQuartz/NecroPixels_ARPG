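; BP_Skeleton is a skeleton character with a Paper2D sprite that activates movement and animation after a short spawn delay.
; Any damage feeds its HealthComponent, and player-instigated damage also plays a hit-stun montage.
; Score and stat managers on the GameState reward hits and kills, varying points by critical or slashing damage and counting critical kills as headshots.
; At zero health it disables movement and collision, then expires shortly after.
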(event `self.ReceiveBeginPlay`
  (bind _sprite (`self.Sprite`))
  (`PaperFlipbookComponent.SetLooping` (`self.Sprite`) false)
  (`KismetSystemLibrary.Delay` 0.8)
  (`ActorComponent.Activate` (`self.CharacterMovement`) false)
  (`ActorComponent.Activate` (`self.PaperAnimationComponent`) false)
  (`PaperFlipbookComponent.SetLooping` _sprite true)
  (`PaperFlipbookComponent.Play` _sprite))

(event `self.HealthComponent.OnHealthZeroed`
  (`ActorComponent.Deactivate` (`self.CharacterMovement`))
  (`self.SetActorEnableCollision` false)
  (`self.SetLifeSpan` 1.0))

(event `self.ReceiveAnyDamage`
  (params (Damage :type "Float (single-precision)") (DamageType :type "DamageType Object Reference") (InstigatedBy :type "Controller Object Reference") (DamageCauser :type "Actor Object Reference"))
  (bind _playerstate (`Controller.PlayerState` InstigatedBy))
  (`/Game/NecroPixelsContent/Components/HealthComponent.DealDamage` (`self.HealthComponent`) Damage)
  (`/Engine/EditorBlueprintResources/StandardMacros.IsValid` _playerstate
    (:`Is Valid`
      (`self.OnDamaged` _playerstate DamageType))))

(fn `OnDamaged`
  (params (Player :type "PlayerState Object Reference") (DamageType :type "DamageType Object Reference"))
  (locals (ScoreManager :type "/Game/NecroPixelsContent/Components/ScoreManagerComponent Object Reference") (ScoreToAward :type Integer :default 10) (StatManager :type "/Game/NecroPixelsContent/Components/StatTrackerManagerComponent Object Reference"))
  (`/Game/NecroPixelsContent/Components/PaperAnimationComponent.PlayMontage` (`self.PaperAnimationComponent`) "/Game/NecroPixelsContent/Character/Skeleton/Flipbooks/Flipbook_Skele_HitStun.Flipbook_Skele_HitStun")
  (set `local.ScoreManager` (`self.GetComponentByClass` (`GameplayStatics.GetGameState`) "/Game/NecroPixelsContent/Components/ScoreManagerComponent.ScoreManagerComponent_C"))
  (set `local.StatManager` (`self.GetComponentByClass` (`GameplayStatics.GetGameState`) "/Game/NecroPixelsContent/Components/StatTrackerManagerComponent.StatTrackerManagerComponent_C"))
  (`|ExecutionSequence`
    (:`then_0`
      (if (`/Game/NecroPixelsContent/Components/HealthComponent.bIsHealthZero` (`self.HealthComponent`))
        (`/Game/NecroPixelsContent/Components/StatTrackerManagerComponent.AddKillToPlayer` (`local.StatManager`) (`local.Player`))
        (cast `/Game/NecroPixelsContent/DamageTypes/DmgType_Critical` (`local.DamageType`)
          (:`then`
            (set `local.ScoreToAward` 100)
            (`/Game/NecroPixelsContent/Components/StatTrackerManagerComponent.AddHeadshotToPlayer` (`local.StatManager`) (`local.Player`)))
          (:`CastFailed`
            (cast `/Game/NecroPixelsContent/DamageTypes/DmgType_Slashing` (`local.DamageType`))
            (set `local.ScoreToAward` 130)))
        (else
          (set `local.ScoreToAward` 10))))
    (:`then_1`
      (`/Game/NecroPixelsContent/Components/ScoreManagerComponent.AwardPlayerScore` (`local.ScoreManager`) (`local.Player`) (`local.ScoreToAward`))
      (`/Game/NecroPixelsContent/Components/StatTrackerManagerComponent.AddScoreToPlayer` (`local.StatManager`) (`local.Player`) (`local.ScoreToAward`)))))

(fn `UserConstructionScript`)