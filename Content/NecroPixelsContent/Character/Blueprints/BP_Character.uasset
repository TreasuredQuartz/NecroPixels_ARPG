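; Player character Blueprint that handles movement, interaction and damage through Enhanced Input and components.
; It registers its input mapping context on BeginPlay, turns the move action into world X/Y movement and sends an interact message to InteractComponent's current actor.
; Incoming damage goes to HealthComponent, whose zero-health event deactivates movement and interaction.
; Getters expose the health and Paper animation components.
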(event `self.ReceiveBeginPlay`
  (`self.AddInputMappingContext`)
  (add `/Game/NecroPixelsContent/Components/HealthComponent.OnHealthZeroed` (`self.HealthComponent`) (delegate `OnDeath`)))

(event `OnDeath`
  (`ActorComponent.Deactivate` (`self.CharacterMovement`))
  (`ActorComponent.Deactivate` (`self.InteractComponent`)))

(event `EnhancedInput|/Game/NecroPixelsContent/Input/IA_Move`
  (params (ActionValue :type "Vector2D Structure") (ElapsedSeconds :type "Float (double-precision)") (TriggeredSeconds :type "Float (double-precision)") (InputAction :type "InputAction Object Reference" :default "/Game/NecroPixelsContent/Input/IA_Move.IA_Move"))
  (bind (_x _y) (`KismetMathLibrary.BreakVector2D` ActionValue))
  (:`Triggered`
    (`self.AddMovementInput` (`KismetMathLibrary.MakeVector` _x _y))))

(event `EnhancedInput|/Game/NecroPixelsContent/Input/IA_Interact`
  (params (ActionValue :type Boolean) (ElapsedSeconds :type "Float (double-precision)") (TriggeredSeconds :type "Float (double-precision)") (InputAction :type "InputAction Object Reference" :default "/Game/NecroPixelsContent/Input/IA_Interact.IA_Interact"))
  (bind _interactibleactor (`/Game/NecroPixelsContent/Components/InteractComponent.InteractibleActor` (`self.InteractComponent`)))
  (:`Triggered`
    (`/Engine/EditorBlueprintResources/StandardMacros.IsValid` _interactibleactor
      (:`Is Valid`
        (message `/Game/NecroPixelsContent/Interfaces/InteractInterface.InteractedWith` _interactibleactor self)))))

(event `self.ReceiveAnyDamage`
  (params (Damage :type "Float (single-precision)") (DamageType :type "DamageType Object Reference") (InstigatedBy :type "Controller Object Reference") (DamageCauser :type "Actor Object Reference"))
  (`/Game/NecroPixelsContent/Components/HealthComponent.DealDamage` (`self.HealthComponent`) Damage))

(fn `AddInputMappingContext`
  (bind _asplayer_controller (cast `PlayerController` (`self.GetController`)))
  (bind _returnvalue (pcsubsystem `EnhancedInputLocalPlayerSubsystem` _asplayer_controller))
  (`/Engine/EditorBlueprintResources/StandardMacros.IsValid` _returnvalue
    (:`Is Valid`
      (`EnhancedInputSubsystemInterface.AddMappingContext` _returnvalue "/Game/NecroPixelsContent/Input/MappingContext.MappingContext" 0 (struct)))))

(fn `GetHealthComponent`
  (returns (OutHealthComponent :type "/Game/NecroPixelsContent/Components/HealthComponent Object Reference"))
  (return (`self.HealthComponent`)))

(fn `GetPaperAnimationComponent`
  (returns (OutPaperAnimationComponent :type "/Game/NecroPixelsContent/Components/PaperAnimationComponent Object Reference"))
  (return (`self.PaperAnimationComponent`)))

(fn `UserConstructionScript`)