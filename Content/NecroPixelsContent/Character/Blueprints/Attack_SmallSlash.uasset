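; Short-lived melee slash hitbox actor that damages anything with a HealthComponent it overlaps, excluding its owner.
; Each target is processed once, taking slashing damage, hit flash, knockback with upward lift and a hit particle, alongside camera shake and audio.
; Hitstop freezes both victim and attacker through their HitstopComponents.
; A brief lifespan ends the attack, and EndPlay reactivates the owner's movement component; the finished-playing binding is never run.
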(event `self.ReceiveBeginPlay`
  (`self.SetLifeSpan` 0.2))

(event `OnFinishedPlaying`
  (`self.SetActorHiddenInGame` true)
  (`self.K2_DestroyActor`))

(event `self.ReceiveActorBeginOverlap`
  (params (OtherActor :type "Actor Object Reference"))
  (if (!= OtherActor (`self.GetOwner`))
    (if (not (`KismetArrayLibrary.Array_Contains` (`self.OverlappedActors`) OtherActor))
      (`KismetArrayLibrary.Array_Add` (`self.OverlappedActors`) OtherActor)
      (`/Engine/EditorBlueprintResources/StandardMacros.IsValid` (`self.GetComponentByClass` OtherActor "/Game/NecroPixelsContent/Components/HealthComponent.HealthComponent_C")
        (:`Is Valid`
          (`GameplayStatics.ApplyDamage` OtherActor 100.0 (`self.GetInstigatorController`) self "/Game/NecroPixelsContent/DamageTypes/DmgType_Slashing.DmgType_Slashing_C")
          (`self.ApplyHitstop` OtherActor 0.15)
          (`self.ApplyHitstop` (`self.GetOwner`) 0.15)
          (`self.ApplyHitFlash` OtherActor 0.15)
          (`self.ApplyKnockback` OtherActor)
          (`self.SpawnHitParticle` OtherActor)
          (`self.CameraShake`)
          (`AudioComponent.Play` (`self.Audio`) 0.0))))))

(event `self.ReceiveEndPlay`
  (params (EndPlayReason :type "EEndPlayReason Enum" :default "Destroyed"))
  (`ActorComponent.Activate` (`self.GetComponentByClass` (`self.GetOwner`) "/Script/Engine.MovementComponent") false))

(fn `ApplyHitFlash`
  (params (Actor :type "Actor Object Reference") (Duration :type "Float (single-precision)"))
  (bind _returnvalue (`self.GetComponentByClass` Actor "/Game/NecroPixelsContent/Components/HitFlashComponent.HitFlashComponent_C"))
  (`/Engine/EditorBlueprintResources/StandardMacros.IsValid` Actor
    (:`Is Valid`
      (`/Engine/EditorBlueprintResources/StandardMacros.IsValid` _returnvalue
        (:`Is Valid`
          (`/Game/NecroPixelsContent/Components/HitFlashComponent.StartFlash` _returnvalue Duration))))))

(fn `ApplyHitstop`
  (params (Actor :type "Actor Object Reference") (Duration :type "Float (single-precision)"))
  (bind _returnvalue (`self.GetComponentByClass` Actor "/Game/NecroPixelsContent/Components/HitstopComponent.HitstopComponent_C"))
  (`/Engine/EditorBlueprintResources/StandardMacros.IsValid` Actor
    (:`Is Valid`
      (`/Engine/EditorBlueprintResources/StandardMacros.IsValid` _returnvalue
        (:`Is Valid`
          (`/Game/NecroPixelsContent/Components/HitstopComponent.StartHitStop` _returnvalue Duration))))))

(fn `ApplyKnockback`
  (params (Actor :type "Actor Object Reference"))
  (bind _returnvalue (`self.GetComponentByClass` Actor "/Script/Engine.CharacterMovementComponent"))
  (`/Engine/EditorBlueprintResources/StandardMacros.IsValid` _returnvalue
    (:`Is Valid`
      (`CharacterMovementComponent.AddImpulse` _returnvalue (+ (* (`KismetMathLibrary.Normal` (- (`self.K2_GetActorLocation` Actor) (`self.K2_GetActorLocation`))) (`self.ForceApplied`)) (* (0.0 0.0 1.0) 1000.0)) false))))

(fn `CameraShake`
  (`GameplayStatics.PlayWorldCameraShake` "/Game/NecroPixelsContent/BP_AttackCameraShake.BP_AttackCameraShake_C" (`SceneComponent.K2_GetComponentLocation` (`self.GetComponentByClass` (`self.GetOwner`) "/Script/Engine.CameraComponent")) 0.0 500.0))

(fn `SpawnHitParticle`
  (params (Actor :type "Actor Object Reference"))
  (`NiagaraFunctionLibrary.SpawnSystemAttached` "/Game/NecroPixelsContent/Character/FX/NS_Slash_HitSkeleton.NS_Slash_HitSkeleton" (`Actor.RootComponent` Actor) "None" (0.0 0.0 0.0) (struct) "SnapToTargetIncludingScale" true))

(fn `UserConstructionScript`
  (`parent.UserConstructionScript`))