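; Slash attack state machine that acts on its owning character, turning melee input into a charged light or heavy attack.
; Tick evaluates Idle, Charging, Light and Heavy states until the owner's health is zeroed, disabling movement outside Idle.
; Light attacks step through timed anticipation, action and recovery, playing flipbook montages and spawning an attached attack actor.
; Heavy attack is a stub returning straight to Idle.
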(event `self.ReceiveBeginPlay`
  (bind _returnvalue (`self.GetComponentByClass` (`self.GetOwner`) "/Game/NecroPixelsContent/Components/HealthComponent.HealthComponent_C"))
  (`/Engine/EditorBlueprintResources/StandardMacros.IsValid` (`self.GetOwner`)
    (:`Is Valid`
      (`|ExecutionSequence`
        (:`then_0`
          (`/Engine/EditorBlueprintResources/StandardMacros.IsValid` _returnvalue
            (:`Is Valid`
              (add `/Game/NecroPixelsContent/Components/HealthComponent.OnHealthZeroed` _returnvalue (delegate `OnHealthZeroed`)))))
        (:`then_1`
          (set `self.PaperAnimationComponent` (`self.GetComponentByClass` (`self.GetOwner`) "/Game/NecroPixelsContent/Components/PaperAnimationComponent.PaperAnimationComponent_C")))))))

(event `OnHealthZeroed`
  (set `self.bIsDead` true))

(event `EnhancedInput|/Game/NecroPixelsContent/Framework/Input/IA_Move`
  (params (ActionValue :type "Vector2D Structure") (ElapsedSeconds :type "Float (double-precision)") (TriggeredSeconds :type "Float (double-precision)") (InputAction :type "InputAction Object Reference" :default "/Game/NecroPixelsContent/Framework/Input/IA_Move.IA_Move"))
  (:`Triggered`
    (set `self.MoveInputDirection` ActionValue)))

(event `EnhancedInput|/Game/NecroPixelsContent/Framework/Input/IA_MeleeAttack`
  (params (ActionValue :type Boolean) (ElapsedSeconds :type "Float (double-precision)") (TriggeredSeconds :type "Float (double-precision)") (InputAction :type "InputAction Object Reference" :default "/Game/NecroPixelsContent/Framework/Input/IA_MeleeAttack.IA_MeleeAttack"))
  (:`Triggered`
    (set `self.bAttackInputDown` ActionValue))
  (:`Completed`
    (set `self.bAttackInputDown` false)))

(event `self.ReceiveTick`
  (params (DeltaSeconds :type "Float (single-precision)"))
  (if (not (`self.bIsDead`))
    (`self.EvaluateState` DeltaSeconds)))

(event `EvaluateState`
  (params (DeltaSeconds :type "Float (double-precision)"))
  (set `self.TimeInState` (+ DeltaSeconds (`self.TimeInState`)))
  (switch `/Game/NecroPixelsContent/Character/Blueprints/Enum_CharacterAttackState` (`self.CharacterState`)
    (:`NewEnumerator3`
      (`self.IdleState`))
    (:`NewEnumerator4`
      (`self.ChargingAttackState`))
    (:`NewEnumerator0`
      (`self.LightAttackState`))
    (:`NewEnumerator1`
      (`self.HeavyAttackState`))))

(event `TransitionToState`
  (params (NewState :type "/Game/NecroPixelsContent/Character/Blueprints/Enum_CharacterAttackState Enum" :default "NewEnumerator3"))
  (if (`self.IsActorTickEnabled`)
    (`self.OnTransitionFromState` NewState)
    (`self.OnTransitionToState` NewState)))

(event `AllowAttacks`
  (`/Engine/EditorBlueprintResources/StandardMacros.Gate` false :!via `Open` :!label _label
    (:`Exit`
      (`self.LightAttackState`))))

(event `PreventAttacks`
  (goto _label :!via `Close`))

(event `StartCooldown`
  (`KismetSystemLibrary.K2_SetTimerDelegate` (`|CreateDelegate` :!event `AllowAttacks`) (`self.Cooldown`)))

(fn `ChargingAttackState`
  (locals (Flipbook_ChargingAttack :type "PaperFlipbook Object Reference" :default "/Script/Paper2D.PaperFlipbook'/Game/NecroPixelsContent/Character/Flipbooks/Flipbook_Cloak_LightAttack_Anticipation.Flipbook_Cloak_LightAttack_Anticipation'"))
  (if (`self.bAttackInputDown`)
    (`/Game/NecroPixelsContent/Components/PaperAnimationComponent.PlayMontage` (`self.PaperAnimationComponent`) (`local.Flipbook_ChargingAttack`))
    (elif (<= (`self.TimeInState`) (`self.HeavyAttackChargeTime`))
      (`self.TransitionToState` "NewEnumerator0")
      (else
        (`self.TransitionToState` "NewEnumerator1")))))

(fn `HeavyAttackState`
  (`self.TransitionToState` "NewEnumerator3"))

(fn `IdleState`
  (if (`self.bAttackInputDown`)
    (`self.TransitionToState` "NewEnumerator4")))

(fn `LightAttackState`
  (locals (TimeInAnticipationState :type "Float (double-precision)" :default 0.0) (TimeInRecoveryState :type "Float (double-precision)" :default 0.55) (Flipbook_LightAttack_Anticipation :type "PaperFlipbook Object Reference" :default "/Script/Paper2D.PaperFlipbook'/Game/NecroPixelsContent/Character/Flipbooks/Flipbook_Cloak_LightAttack_Anticipation.Flipbook_Cloak_LightAttack_Anticipation'") (Flipbook_LightAttack_Action :type "PaperFlipbook Object Reference" :default "/Script/Paper2D.PaperFlipbook'/Game/NecroPixelsContent/Character/Flipbooks/Flipbook_Cloak_LightAttack_Action.Flipbook_Cloak_LightAttack_Action'") (Flipbook_LightAttack_Recovery :type "PaperFlipbook Object Reference" :default "/Script/Paper2D.PaperFlipbook'/Game/NecroPixelsContent/Character/Flipbooks/Flipbook_Cloak_LightAttack_Recovery.Flipbook_Cloak_LightAttack_Recovery'"))
  (bind _returnvalue (`self.GetOwner`))
  (bind _returnvalue_2 (`self.GetComponentByClass` _returnvalue "/Script/Paper2D.PaperFlipbookComponent"))
  (bind (_returnvalue_location _returnvalue_rotation _returnvalue_scale) (`KismetMathLibrary.BreakTransform` (`SceneComponent.K2_GetComponentToWorld` _returnvalue_2)))
  (switch `/Game/NecroPixelsContent/Character/Blueprints/Enum_SubAttackState` (`self.CurrentAttackState`)
    (:`NewEnumerator0`
      (set `self.CurrentAttackState` "NewEnumerator1"))
    (:`NewEnumerator1`
      (if (>= (`self.TimeInState`) (`local.TimeInAnticipationState`))
        (`/Game/NecroPixelsContent/Components/PaperAnimationComponent.PlayMontage` (`self.PaperAnimationComponent`) (`local.Flipbook_LightAttack_Action`))
        (set `self.CurrentAttackState` "NewEnumerator2")))
    (:`NewEnumerator2`
      (`/Engine/EditorBlueprintResources/StandardMacros.IsValid` _returnvalue_2
        (:`Is Valid`
          (bind _returnvalue_3 (`|SpawnActorFromClass` (`self.AtackInstanceClass`) (`KismetMathLibrary.MakeTransform` (+ _returnvalue_location (0.0 0.0 5.0)) _returnvalue_rotation _returnvalue_scale) "AlwaysSpawn" "MultiplyWithRoot" _returnvalue (cast `Pawn` _returnvalue :!pure true)))
          (`self.K2_AttachToActor` _returnvalue_3 (`self.GetOwner`) "None" "KeepWorld" "KeepWorld" "KeepWorld" true)
          (`/Game/NecroPixelsContent/Components/PaperAnimationComponent.PlayMontage` (`self.PaperAnimationComponent`) (`local.Flipbook_LightAttack_Recovery`))
          (set `self.CurrentAttackState` "NewEnumerator3"))))
    (:`NewEnumerator3`
      (if (>= (- (`self.TimeInState`) (`local.TimeInAnticipationState`)) (`local.TimeInRecoveryState`))
        (`self.TransitionToState` "NewEnumerator3")))))

(fn `OnTransitionFromState`
  (params (NextState :type "/Game/NecroPixelsContent/Character/Blueprints/Enum_CharacterAttackState Enum" :default "NewEnumerator3"))
  (bind _returnvalue (`self.GetComponentByClass` (`self.GetOwner`) "/Script/Engine.CharacterMovementComponent"))
  (switch `/Game/NecroPixelsContent/Character/Blueprints/Enum_CharacterAttackState` (`self.CharacterState`)
    (:`NewEnumerator3`
      (`MovementComponent.StopMovementImmediately` _returnvalue)
      (`CharacterMovementComponent.DisableMovement` _returnvalue))))

(fn `OnTransitionToState`
  (params (NewState :type "/Game/NecroPixelsContent/Character/Blueprints/Enum_CharacterAttackState Enum" :default "NewEnumerator3"))
  (set `self.CharacterState` NewState)
  (set `self.TimeInState` 0.0)
  (set `self.CurrentAttackState` "NewEnumerator0")
  (switch `/Game/NecroPixelsContent/Character/Blueprints/Enum_CharacterAttackState` (`self.CharacterState`)
    (:`NewEnumerator3`
      (`CharacterMovementComponent.SetMovementMode` (`self.GetComponentByClass` (`self.GetOwner`) "/Script/Engine.CharacterMovementComponent") "MOVE_Walking" 0))))

(fn `UserConstructionScript`)