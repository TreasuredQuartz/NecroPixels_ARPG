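; Character state machine that drives melee-style attack states for a Paper2D character, caching health, animation and attack components and halting evaluation on death.
; Each tick runs the current state: Idle consumes attack input into Light Attack, while Charging picks light or heavy by hold time.
; Light Attack steps through timed anticipation, action and recovery, playing flipbook montages and spawning an attached attack actor.
; Transitions lock movement leaving Idle and restore walking on return; Heavy Attack is empty.
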(event `OnHealthZeroed`
  (set `self.bIsDead` true))

(event `self.InitializeState_BP`
  (bind _returnvalue (`self.GetComponentByClass` (`self.OwningActor`) "/Game/NecroPixelsContent/Components/HealthComponent.HealthComponent_C"))
  (bind _returnvalue_2 (`self.GetComponentByClass` (`self.OwningActor`) "/Game/NecroPixelsContent/Components/AttackComponent.AttackComponent_C"))
  (`/Engine/EditorBlueprintResources/StandardMacros.IsValid` (`self.OwningActor`)
    (:`Is Valid`
      (`|ExecutionSequence`
        (:`then_0`
          (`/Engine/EditorBlueprintResources/StandardMacros.IsValid` _returnvalue
            (:`Is Valid`
              (add `/Game/NecroPixelsContent/Components/HealthComponent.OnHealthZeroed` _returnvalue (delegate `OnHealthZeroed`)))))
        (:`then_1`
          (set `self.PaperAnimationComponent` (`self.GetComponentByClass` (`self.OwningActor`) "/Game/NecroPixelsContent/Components/PaperAnimationComponent.PaperAnimationComponent_C")))
        (:`then_2`
          (`/Engine/EditorBlueprintResources/StandardMacros.IsValid` _returnvalue_2
            (:`Is Valid`
              (set `self.AttackComponent` _returnvalue_2))))))))

(event `self.EvaluateStateMachine_BP`
  (params (DeltaTime :type "Float (single-precision)"))
  (set `self.TimeInState` (+ DeltaTime (`self.TimeInState`)))
  (if (not (`self.bIsDead`))
    (`|ExecutionSequence`
      (:`then_0`
        (`/Engine/EditorBlueprintResources/StandardMacros.IsValid` (`self.CurrentNode`)
          (:`Is Valid`
            (`KismetSystemLibrary.PrintString` "Hello"))
          (:`Is Not Valid`
            (`KismetSystemLibrary.PrintString` "Undefined"))))
      (:`then_1`
        (switch `/Game/NecroPixelsContent/Character/Blueprints/Attacks/Enum_CharacterAttackState` (`self.CharacterState`)
          (:`NewEnumerator3`
            (`self.IdleState`))
          (:`NewEnumerator4`
            (`self.ChargingAttackState`))
          (:`NewEnumerator0`
            (`self.LightAttackState`))
          (:`NewEnumerator1`
            (`self.HeavyAttackState`)))))))

(event `TransitionToState`
  (params (NewState :type "/Game/NecroPixelsContent/Character/Blueprints/Attacks/Enum_CharacterAttackState Enum" :default "NewEnumerator3"))
  (`self.OnTransitionFromState` NewState)
  (`self.OnTransitionToState` NewState))

(fn `ChargingAttackState`
  (locals (HeavyAttackChargeTime :type "Float (single-precision)") (Flipbook_ChargingAttack :type "PaperFlipbook Object Reference" :default "/Script/Paper2D.PaperFlipbook'/Game/NecroPixelsContent/Character/Flipbooks/Flipbook_Cloak_LightAttack_Anticipation.Flipbook_Cloak_LightAttack_Anticipation'"))
  (if (`self.bAttackInputDown`)
    (`/Game/NecroPixelsContent/Components/PaperAnimationComponent.PlayMontage` (`self.PaperAnimationComponent`) (`local.Flipbook_ChargingAttack`))
    (elif (<= (`self.TimeInState`) (`local.HeavyAttackChargeTime`))
      (`self.TransitionToState` "NewEnumerator0")
      (else
        (`self.TransitionToState` "NewEnumerator1")))))

(fn `HeavyAttackState`)

(fn `IdleState`
  (bind _attackcomponent (`self.AttackComponent`))
  (if (`/Game/NecroPixelsContent/Components/AttackComponent.bAttackInputDown` _attackcomponent)
    (`/Game/NecroPixelsContent/Components/AttackComponent.ConsumeAttackInput` _attackcomponent)
    (`self.TransitionToState` "NewEnumerator0")))

(fn `LightAttackState`
  (locals (AttackInstanceClass :type "/Game/NecroPixelsContent/AttackStateMachineGraph/AttackInstance Class Reference" :default "/Script/Engine.BlueprintGeneratedClass'/Game/NecroPixelsContent/Character/Blueprints/Attacks/Attack_Light01_Slash.Attack_Light01_Slash_C'") (Flipbook_LightAttack_Recovery :type "PaperFlipbook Object Reference" :default "/Script/Paper2D.PaperFlipbook'/Game/NecroPixelsContent/Character/Flipbooks/Flipbook_Cloak_LightAttack_Recovery.Flipbook_Cloak_LightAttack_Recovery'") (Flipbook_LightAttack_Action :type "PaperFlipbook Object Reference" :default "/Script/Paper2D.PaperFlipbook'/Game/NecroPixelsContent/Character/Flipbooks/Flipbook_Cloak_LightAttack01.Flipbook_Cloak_LightAttack01'") (TimeInAnticipationState :type "Float (double-precision)") (TimeInRecoveryState :type "Float (double-precision)" :default 0.55))
  (bind _aspawn (cast `Pawn` (`self.OwningActor`) :!pure true))
  (bind (_returnvalue_location _returnvalue_rotation _returnvalue_scale) (`KismetMathLibrary.BreakTransform` (`SceneComponent.K2_GetComponentToWorld` (`self.GetComponentByClass` (`self.OwningActor`) "/Script/Paper2D.PaperFlipbookComponent"))))
  (switch `/Game/NecroPixelsContent/Character/Blueprints/Attacks/Enum_SubAttackState` (`self.CurrentAttackState`)
    (:`NewEnumerator0`
      (set `self.CurrentAttackState` "NewEnumerator1"))
    (:`NewEnumerator1`
      (if (>= (`self.TimeInState`) (`local.TimeInAnticipationState`))
        (`/Game/NecroPixelsContent/Components/PaperAnimationComponent.PlayMontage` (`self.PaperAnimationComponent`) (`local.Flipbook_LightAttack_Action`))
        (set `self.CurrentAttackState` "NewEnumerator2")))
    (:`NewEnumerator2`
      (bind _returnvalue (`|SpawnActorFromClass` (`local.AttackInstanceClass`) (`KismetMathLibrary.MakeTransform` (+ _returnvalue_location (0.0 0.0 5.0)) _returnvalue_rotation _returnvalue_scale) "AlwaysSpawn" "MultiplyWithRoot" _aspawn _aspawn))
      (`self.K2_AttachToActor` _returnvalue (`self.OwningActor`) "None" "KeepWorld" "KeepWorld" "KeepWorld" true)
      (`/Game/NecroPixelsContent/Components/PaperAnimationComponent.PlayMontage` (`self.PaperAnimationComponent`) (`local.Flipbook_LightAttack_Recovery`))
      (set `self.CurrentAttackState` "NewEnumerator3"))
    (:`NewEnumerator3`
      (if (>= (- (`self.TimeInState`) (`local.TimeInAnticipationState`)) (`local.TimeInRecoveryState`))
        (`self.TransitionToState` "NewEnumerator3")))))

(fn `OnTransitionFromState`
  (params (NextState :type "/Game/NecroPixelsContent/Character/Blueprints/Attacks/Enum_CharacterAttackState Enum" :default "NewEnumerator3"))
  (bind _returnvalue (`self.GetComponentByClass` (`self.OwningActor`) "/Script/Engine.CharacterMovementComponent"))
  (switch `/Game/NecroPixelsContent/Character/Blueprints/Attacks/Enum_CharacterAttackState` (`self.CharacterState`)
    (:`NewEnumerator3`
      (`MovementComponent.StopMovementImmediately` _returnvalue)
      (`CharacterMovementComponent.DisableMovement` _returnvalue))))

(fn `OnTransitionToState`
  (params (NewState :type "/Game/NecroPixelsContent/Character/Blueprints/Attacks/Enum_CharacterAttackState Enum" :default "NewEnumerator3"))
  (set `self.CharacterState` NewState)
  (set `self.TimeInState` 0.0)
  (set `self.CurrentAttackState` "NewEnumerator0")
  (switch `/Game/NecroPixelsContent/Character/Blueprints/Attacks/Enum_CharacterAttackState` (`self.CharacterState`)
    (:`NewEnumerator3`
      (`CharacterMovementComponent.SetMovementMode` (`self.GetComponentByClass` (`self.OwningActor`) "/Script/Engine.CharacterMovementComponent") "MOVE_Walking" 0))))

(fn `UserConstructionScript`)