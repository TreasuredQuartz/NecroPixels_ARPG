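; Short-lived melee slash attack actor that plays its flipbook once, then hides and destroys itself.
; On overlap it damages each non-owner actor with a HealthComponent only once, up to a maximum enemy count, using slashing damage.
; Each hit adds hitstop on victim and owner through their components, plus a hit flash, knockback with upward lift, an attached Niagara effect, camera shake and audio.
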(event `self.ReceiveBeginPlay`
  (bind _paperflipbook (`self.PaperFlipbook`))
  (add `PaperFlipbookComponent.OnFinishedPlaying` (`self.PaperFlipbook`) (delegate `OnFinishedPlaying`))
  (`PaperFlipbookComponent.SetLooping` _paperflipbook false)
  (`PaperFlipbookComponent.Play` _paperflipbook))

(event `OnFinishedPlaying`
  (`self.SetActorHiddenInGame` true)
  (`self.K2_DestroyActor`))

(event `self.ReceiveActorBeginOverlap`
  (params (OtherActor :type "Actor Object Reference"))
  (bind _bshoulddamage (`self.ShouldDamageActor` OtherActor))
  (if _bshoulddamage
    (`GameplayStatics.ApplyDamage` OtherActor (`self.BaseDamage`) (`self.GetInstigatorController`) self "/Game/NecroPixelsContent/DamageTypes/DmgType_Slashing.DmgType_Slashing_C")
    (`self.ApplyHitstop` OtherActor 0.15)
    (`self.ApplyHitstop` (`self.GetOwner`) 0.15)
    (`self.ApplyHitFlash` OtherActor 0.15)
    (`self.ApplyKnockback` OtherActor)
    (`self.SpawnHitParticle` OtherActor)
    (`self.CameraShake`)
    (`AudioComponent.Play` (`self.Audio`) 0.0)))

(fn `ApplyHitFlash`
  (params (Actor :type "Actor Object Reference") (Duration :type "Float (single-precision)"))
  (bind _returnvalue (`self.GetComponentByClass` Actor "/Game/NecroPixelsContent/Components/HitFlashComponent.HitFlashComponent_C"))
  (`/Engine/EditorBlueprintResources/StandardMacros.IsValid` Actor
    (:`Is Valid`
      (`/Engine/EditorBlueprintResources/StandardMacros.IsValid` _returnvalue
        (:`Is Valid`
          (`/Game/NecroPixelsContent/Components/HitFlashComponent.StartFlash` _returnvalue Duration))))))

(fn `ApplyHitstop`
  (params (Actor :type "Actor Object Reference") (Duration :type "Float (single-precision)"))
  (bind _returnvalue (`self.GetComponentByClass` Actor "/Game/NecroPixelsContent/Components/HitstopComponent.HitstopComponent_C"))
  (`/Engine/EditorBlueprintResources/StandardMacros.IsValid` Actor
    (:`Is Valid`
      (`/Engine/EditorBlueprintResources/StandardMacros.IsValid` _returnvalue
        (:`Is Valid`
          (`/Game/NecroPixelsContent/Components/HitstopComponent.StartHitStop` _returnvalue Duration))))))

(fn `ApplyKnockback`
  (params (Actor :type "Actor Object Reference"))
  (bind _returnvalue (`self.GetComponentByClass` Actor "/Script/Engine.CharacterMovementComponent"))
  (`/Engine/EditorBlueprintResources/StandardMacros.IsValid` _returnvalue
    (:`Is Valid`
      (`CharacterMovementComponent.AddImpulse` _returnvalue (+ (* (`KismetMathLibrary.Normal` (- (`self.K2_GetActorLocation` Actor) (`self.K2_GetActorLocation`))) (`self.ForceApplied`)) (* (0.0 0.0 1.0) 1000.0)) false))))

(fn `CameraShake`
  (`GameplayStatics.PlayWorldCameraShake` "/Game/NecroPixelsContent/BP_AttackCameraShake.BP_AttackCameraShake_C" (`SceneComponent.K2_GetComponentLocation` (`self.GetComponentByClass` (`self.GetOwner`) "/Script/Engine.CameraComponent")) 0.0 500.0))

(fn `ShouldDamageActor`
  (params (Actor :type "Actor Object Reference"))
  (returns (bShouldDamage :type Boolean))
  ;[1 1 1] Is this not self-harm?
  (if (!= (`local.Actor`) (`self.GetOwner`))
    ;[1 1 1] Should hit the same actor multiple times?
    (if (not (`KismetArrayLibrary.Array_Contains` (`self.OverlappedActors`) (`local.Actor`)))
      (`KismetArrayLibrary.Array_Add` (`self.OverlappedActors`) (`local.Actor`))
      ;[1 1 1] Does this actor have health?
      (`/Engine/EditorBlueprintResources/StandardMacros.IsValid` (`self.GetComponentByClass` (`local.Actor`) "/Game/NecroPixelsContent/Components/HealthComponent.HealthComponent_C")
        (:`Is Valid`
          ;[1 1 1] Should Hit Multiple Enemies?
          (if (< (`self.DamagedEnemyCount`) (`self.MaxDamagedEnemyCount`))
            (`/Engine/EditorBlueprintResources/StandardMacros.IncrementInt` (`self.DamagedEnemyCount`)
              (:`  `
                ;[0 1 0.135] Yes.
                (return true)))
            (else
              _)))
        (:`Is Not Valid`
          _))))
  ;[1 0 0] No.
  (return false))

(fn `SpawnHitParticle`
  (params (Actor :type "Actor Object Reference"))
  (`NiagaraFunctionLibrary.SpawnSystemAttached` "/Game/NecroPixelsContent/Character/FX/NS_Slash_HitSkeleton.NS_Slash_HitSkeleton" (`Actor.RootComponent` Actor) "None" (0.0 0.0 0.0) (struct) "SnapToTargetIncludingScale" true))

(fn `UserConstructionScript`
  (`parent.UserConstructionScript`))