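; Forest Blueprint that fills a box volume with a grid of tree sprites.
; The construction script calls InitializeForestTiles, which clears the PaperGroupedSprite and adds rotated TreeSprite instances spaced by placement width and height across the box extent.
; Odd columns shift by half a cell in Y for a staggered layout and take a small Z offset that separates them in depth from even columns.
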(fn `InitializeForestTiles`
  (bind (_boxextent_x _boxextent_y) (`KismetMathLibrary.BreakVector` (`BoxComponent.BoxExtent` (`self.Box`))))
  (bind _returnvalue (`KismetMathLibrary.FTrunc` (/ _boxextent_y (`self.PlacementHeight`))))
  (bind _returnvalue_2 (`KismetMathLibrary.FTrunc` (/ _boxextent_x (`self.PlacementWidth`))))
  (`PaperGroupedSpriteComponent.ClearInstances` (`self.PaperGroupedSprite`))
  (for _index (range (- 0 _returnvalue_2) (+ _returnvalue_2 1))
    (for _index_2 (range (- 0 _returnvalue) (+ _returnvalue 1))
      (bind _returnvalue_3 (mod _index 2))
      (`PaperGroupedSpriteComponent.AddInstance` (`self.PaperGroupedSprite`) (`KismetMathLibrary.MakeTransform` (`KismetMathLibrary.MakeVector` (* _index (`self.PlacementWidth`)) (+ (* _index_2 (`self.PlacementHeight`)) (* (`self.PlacementHeight`) 0.5 _returnvalue_3)) (`KismetMathLibrary.Conv_IntToDouble` _returnvalue_3)) (struct :`Roll` -90.0)) (`self.TreeSprite`) false (struct :`R` 1.0 :`G` 1.0 :`B` 1.0 :`A` 1.0)))))

(fn `UserConstructionScript`
  (`self.InitializeForestTiles`))