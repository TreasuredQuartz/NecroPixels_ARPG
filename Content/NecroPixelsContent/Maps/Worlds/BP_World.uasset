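; BP_World is an interactable world actor that sends the interacting actor to LevelTransitionComponent for level travel.
; Overlapping its interact sphere registers it with the actor's InteractComponent, and leaving clears it.
; The construction script builds a "Gummi Road" spline by projecting Points onto a ring at the sphere radius, half a radius below center.
; With three or more points, it adds a spline mesh per segment, plus one closing closed loops.
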(event `/Game/NecroPixelsContent/Interfaces/InteractInterface.InteractedWith`
  (params (OtherActor :type "Actor Object Reference"))
  (`/Game/NecroPixelsContent/Components/Gamemodes/LevelTransitionComponent.LevelTravel` (`self.LevelTransitionComponent`) OtherActor))

(event `self.Sphere_Interact.OnComponentBeginOverlap`
  (params (OverlappedComponent :type "PrimitiveComponent Object Reference") (OtherActor :type "Actor Object Reference") (OtherComp :type "PrimitiveComponent Object Reference") (OtherBodyIndex :type Integer) (bFromSweep :type Boolean) (SweepResult :type "HitResult Structure (by ref)"))
  (bind _returnvalue (`self.GetComponentByClass` OtherActor "/Game/NecroPixelsContent/Components/Pawns/InteractComponent.InteractComponent_C"))
  (`/Engine/EditorBlueprintResources/StandardMacros.IsValid` _returnvalue
    (:`Is Valid`
      (`/Game/NecroPixelsContent/Components/Pawns/InteractComponent.SetInteractibleActor` _returnvalue self))))

(event `self.Sphere_Interact.OnComponentEndOverlap`
  (params (OverlappedComponent :type "PrimitiveComponent Object Reference") (OtherActor :type "Actor Object Reference") (OtherComp :type "PrimitiveComponent Object Reference") (OtherBodyIndex :type Integer))
  (bind _returnvalue (`self.GetComponentByClass` OtherActor "/Game/NecroPixelsContent/Components/Pawns/InteractComponent.InteractComponent_C"))
  (`/Engine/EditorBlueprintResources/StandardMacros.IsValid` _returnvalue
    (:`Is Valid`
      (`/Game/NecroPixelsContent/Components/Pawns/InteractComponent.SetInteractibleActor` _returnvalue null))))

(fn `AddSplineMesh`
  (params (StartPos :type "Vector Structure") (StartTangent :type "Vector Structure") (EndPos :type "Vector Structure") (EndTangent :type "Vector Structure"))
  (bind _returnvalue (`AddComponent|NODE_AddSplineMeshComponent-0`))
  (`KismetArrayLibrary.Array_Add` (`self.SplineMeshes`) _returnvalue)
  (`SplineMeshComponent.SetStartAndEnd` _returnvalue StartPos StartTangent EndPos EndTangent true))

(fn `CreateSplineMesh`
  (params (Spline :type "SplineComponent Object Reference"))
  (locals (StartIndex :type Integer) (EndIndex :type Integer) (StartPos :type "Vector Structure") (StartTan :type "Vector Structure") (EndPos :type "Vector Structure") (EndTan :type "Vector Structure"))
  (bind _returnvalue (`SplineComponent.GetNumberOfSplinePoints` (`local.Spline`)))
  (if (>= _returnvalue 3)
    (`KismetArrayLibrary.Array_Clear` (`self.SplineMeshes`))
    (for _index (range (+ (- _returnvalue 2) 1))
      (set `local.StartIndex` _index)
      (set `local.EndIndex` (+ (`local.StartIndex`) 1))
      (set `local.StartPos` (`SplineComponent.GetLocationAtSplinePoint` (`local.Spline`) (`local.StartIndex`) "Local") :!label _label)
      (set `local.StartTan` (`SplineComponent.GetTangentAtSplinePoint` (`local.Spline`) (`local.StartIndex`) "Local"))
      (set `local.EndPos` (`SplineComponent.GetLocationAtSplinePoint` (`local.Spline`) (`local.EndIndex`) "Local"))
      (set `local.EndTan` (`SplineComponent.GetTangentAtSplinePoint` (`local.Spline`) (`local.EndIndex`) "Local"))
      (`self.AddSplineMesh` (`local.StartPos`) (`local.StartTan`) (`local.EndPos`) (`local.EndTan`)))
    (if (`SplineComponent.IsClosedLoop` (`local.Spline`))
      (set `local.StartIndex` (- (`SplineComponent.GetNumberOfSplinePoints` (`local.Spline`)) 1))
      (set `local.EndIndex` 0)
      (goto _label))))

(fn `CreateSplinePoint`
  (locals (Radius :type "Float (single-precision)" :default 0.0) (Points :type "Array of Vector2D Structure"))
  (set `local.Radius` (`SphereComponent.SphereRadius` (`self.Sphere_Interact`)))
  (bind _returnvalue (`AddComponent|NODE_AddSplineComponent-0`))
  (set `self.SplineComp_GummiRoad` _returnvalue)
  (`SplineComponent.ClearSplinePoints` (`self.SplineComp_GummiRoad`) true)
  (for _array_element (`local.Points`)
    (`SplineComponent.AddSplinePoint` (`self.SplineComp_GummiRoad`) (`KismetMathLibrary.Conv_Vector2DToVector` (* (`KismetMathLibrary.Normal2D` _array_element) (`local.Radius`)) (* (`local.Radius`) -0.5)) "Local" true)))

(fn `GetInteractionInfo`
  (returns (DisplayString :type String))
  (return ""))

(fn `UserConstructionScript`
  (`self.CreateSplinePoint`)
  (`self.CreateSplineMesh` (`self.SplineComp_GummiRoad`)))