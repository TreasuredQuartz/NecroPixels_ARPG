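; BP_GummiRoad is a spline-driven road actor that lays spline mesh segments along its Spline component.
; CreateSplineMesh runs in the construction script and again one tick after BeginPlay, requiring at least three spline points.
; It passes local positions and tangents of each point pair to AddSplineMesh, adding a closing segment for looped splines.
; The rebuild clears the SplineMeshes array without explicitly destroying existing components.
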(event `self.ReceiveBeginPlay`
  (`KismetSystemLibrary.DelayUntilNextTick`)
  (`self.CreateSplineMesh`))

(fn `AddSplineMesh`
  (params (StartPos :type "Vector Structure") (StartTangent :type "Vector Structure") (EndPos :type "Vector Structure") (EndTangent :type "Vector Structure"))
  (bind _returnvalue (`AddComponent|NODE_AddSplineMeshComponent-0`))
  (`KismetArrayLibrary.Array_Add` (`self.SplineMeshes`) _returnvalue)
  (`SplineMeshComponent.SetStartAndEnd` _returnvalue StartPos StartTangent EndPos EndTangent true))

(fn `CreateSplineMesh`
  (locals (StartPos :type "Vector Structure" :default (0.0 0.0 0.0)) (StartTan :type "Vector Structure" :default (0.0 0.0 0.0)) (EndPos :type "Vector Structure" :default (0.0 0.0 0.0)) (EndTan :type "Vector Structure" :default (0.0 0.0 0.0)) (StartIndex :type Integer) (EndIndex :type Integer))
  (bind _returnvalue (`SplineComponent.GetNumberOfSplinePoints` (`self.Spline`)))
  (if (>= _returnvalue 3)
    (`KismetArrayLibrary.Array_Clear` (`self.SplineMeshes`))
    (for _index (range (+ (- _returnvalue 2) 1))
      (set `local.StartIndex` _index)
      (set `local.EndIndex` (+ (`local.StartIndex`) 1))
      (set `local.StartPos` (`SplineComponent.GetLocationAtSplinePoint` (`self.Spline`) (`local.StartIndex`) "Local") :!label _label)
      (set `local.StartTan` (`SplineComponent.GetTangentAtSplinePoint` (`self.Spline`) (`local.StartIndex`) "Local"))
      (set `local.EndPos` (`SplineComponent.GetLocationAtSplinePoint` (`self.Spline`) (`local.EndIndex`) "Local"))
      (set `local.EndTan` (`SplineComponent.GetTangentAtSplinePoint` (`self.Spline`) (`local.EndIndex`) "Local"))
      (`self.AddSplineMesh` (`local.StartPos`) (`local.StartTan`) (`local.EndPos`) (`local.EndTan`)))
    (if (`SplineComponent.IsClosedLoop` (`self.Spline`))
      (set `local.StartIndex` (- (`SplineComponent.GetNumberOfSplinePoints` (`self.Spline`)) 1))
      (set `local.EndIndex` 0)
      (goto _label))))

(fn `UserConstructionScript`
  (`self.CreateSplineMesh`))