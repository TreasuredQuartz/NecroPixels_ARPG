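; Station platform actor for the Dive to the Heart world: a round glass spire built from Paper2D sprites, with a platform on top.
; The construction script runs CreateSides to stack rings of side sprites around Radius to fit Height, then moves the platform to Height.
; Each panel faces the center with alternating roll, using grouped sprite instances with a distinct top-row sprite.
; Top-row transforms also place instanced barrier meshes, raised and nudged outward.
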(fn `CreateSides`
  (locals (SideTopTransforms :type "Array of Transform Structure") (SideTransforms :type "Array of Transform Structure") (MaxSides :type Integer) (MaxHeightIndex :type Integer :default 0) (CurIndex :type Integer) (CurHeightIndex :type Integer) (SideSpriteHeight :type "Float (double-precision)" :default 50.0) (SideTopSpriteHeight :type "Float (double-precision)" :default 166.0) (HeightRemainder :type "Float (double-precision)" :default 0.0) (CurIndexNormalizedLoc :type "Vector Structure") (CurIndexRealLoc :type "Vector Structure") (CurIndexScale :type "Vector Structure" :default (1.0 1.0 1.0)) (CurIndexRotation :type "Rotator Structure" :default (struct)) (IsTopLayer :type Boolean))
  (bind _sidespriteheight (`local.SideSpriteHeight`))
  (bind (_remainder _returnvalue) (`KismetMathLibrary.FMod` (- (`self.Height`) (`local.SideTopSpriteHeight`)) (`local.SideSpriteHeight`)))
  (`PaperGroupedSpriteComponent.ClearInstances` (`self.PaperGroupedSprite_Spire`))
  (if (> (`self.Sides`) 0)
    (set `local.MaxSides` (- (`self.Sides`) 1))
    (if (> (- (`self.Height`) (`local.SideTopSpriteHeight`)) 0.0)
      (set `local.HeightRemainder` _remainder)
      (set `local.MaxHeightIndex` _returnvalue)
      (for _index (range (+ (`local.MaxHeightIndex`) 1))
        (set `local.CurHeightIndex` _index)
        (for _index_2 (range (+ (`local.MaxSides`) 1)) :!label _label
          (set `local.CurIndex` _index_2)
          (set `local.IsTopLayer` (>= (`local.CurHeightIndex`) (`local.MaxHeightIndex`)))
          (if (< (`local.CurIndex`) (`local.MaxSides`))
            (set `local.CurIndexNormalizedLoc` (* (`KismetMathLibrary.RotateAngleAxis` (`self.GetActorForwardVector`) (* (/ (`KismetMathLibrary.Conv_IntToDouble` (`local.CurIndex`)) (`local.MaxSides`)) 360.0) (`self.GetActorUpVector`)) (`self.Radius`)))
            (set `local.CurIndexRealLoc` (+ (`local.CurIndexNormalizedLoc`) (`KismetMathLibrary.MakeVector` 0.0 0.0 (+ (`local.HeightRemainder`) (- (`self.Height`) (+ (* (`KismetMathLibrary.SelectFloat` (+ _sidespriteheight 39.0) _sidespriteheight (`local.IsTopLayer`)) (- (- (`local.MaxHeightIndex`) 1) (`local.CurHeightIndex`))) (`local.SideTopSpriteHeight`)))))))
            (set `local.CurIndexRotation` (`KismetMathLibrary.ComposeRotators` (`KismetMathLibrary.FindLookAtRotation` (`local.CurIndexNormalizedLoc`) (`KismetMathLibrary.Vector_Zero`)) (`KismetMathLibrary.SelectRotator` (struct :`Yaw` 90.0) (struct :`Yaw` -90.0) (== (mod (`local.CurIndex`) 2) 0))))
            (if (`local.IsTopLayer`)
              (`KismetArrayLibrary.Array_Add` (`local.SideTopTransforms`) (`KismetMathLibrary.MakeTransform` (`local.CurIndexRealLoc`) (`local.CurIndexRotation`) (`local.CurIndexScale`)))
              (else
                (`KismetArrayLibrary.Array_Add` (`local.SideTransforms`) (`KismetMathLibrary.MakeTransform` (`local.CurIndexRealLoc`) (`local.CurIndexRotation`) (`local.CurIndexScale`))))))))
      (for (_array_element _array_index) (`local.SideTopTransforms`)
        (`PaperGroupedSpriteComponent.AddInstance` (`self.PaperGroupedSprite_Spire`) _array_element "/Game/NecroPixelsContent/Maps/Worlds/DiveToTheHeart/Textures/S_Station_Glass_Top.S_Station_Glass_Top" false (struct :`R` 1.0 :`G` 1.0 :`B` 1.0 :`A` 1.0))
        (bind _returnvalue_2 (+ (.location _array_element) (0.0 0.0 100.0)))
        (`InstancedStaticMeshComponent.AddInstance` (`self.InstancedStaticMesh_Barrier`) (`KismetMathLibrary.MakeTransform` (+ _returnvalue_2 (* (`KismetMathLibrary.Normal2D` (`KismetMathLibrary.MakeVector2D` (.x _returnvalue_2) (.y _returnvalue_2))) 2.3)) (`KismetMathLibrary.MakeRotator` (+ (.roll (.rotation _array_element)) (`KismetMathLibrary.SelectFloat` -90.0 -90.0 (== (mod _array_index 2) 0))) (.pitch (.rotation _array_element)) (.yaw (.rotation _array_element))) (`KismetMathLibrary.MakeVector` 0.65 0.65 0.65)) false))
      (for _array_element_2 (`local.SideTransforms`)
        (`PaperGroupedSpriteComponent.AddInstance` (`self.PaperGroupedSprite_Spire`) _array_element_2 "/Game/NecroPixelsContent/Maps/Worlds/DiveToTheHeart/Textures/S_Station_Glass_Body.S_Station_Glass_Body" false (struct :`R` 1.0 :`G` 1.0 :`B` 1.0 :`A` 1.0)))
      (else
        (goto _label)))))

(fn `UserConstructionScript`
  (`self.CreateSides`)
  (`SceneComponent.K2_SetRelativeLocation` (`self.PaperSprite_Platform`) (`KismetMathLibrary.MakeVector` 0.0 0.0 (`self.Height`)) false true))