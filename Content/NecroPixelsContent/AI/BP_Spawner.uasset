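; BP_Spawner is a spawner actor that creates instances of a configurable SpawnClass inside its Box volume.
; ShouldSpawn simply returns the IsSpawnerActive flag, and nothing in this file calls it or SpawnActor.
; SpawnActor picks a random point around the actor using half the box's scaled extent, always spawns regardless of collision, and returns the new actor.
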(fn `ShouldSpawn`
  (returns (ReturnValue :type Boolean))
  (return (`self.bIsSpawnerActive`)))

(fn `SpawnActor`
  (returns (ReturnValue :type "Actor Object Reference"))
  (bind _returnvalue (`|SpawnActorFromClass` (`self.SpawnClass`) (`KismetMathLibrary.MakeTransform` (`KismetMathLibrary.RandomPointInBoundingBox` (`self.K2_GetActorLocation`) (/ (`BoxComponent.GetScaledBoxExtent` (`self.Box`)) 2))) "AlwaysSpawn" "MultiplyWithRoot" null null))
  (return _returnvalue))

(fn `UserConstructionScript`)