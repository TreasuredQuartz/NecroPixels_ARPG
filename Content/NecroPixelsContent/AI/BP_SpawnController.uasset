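; BP_SpawnController refills a set of spawners with actors in waves, starting a new wave once the previous one is gone.
; A looping timer checks the live count and, when it reaches zero, triggers every valid spawner in its list.
; Each spawned actor adds to the count, and its HealthComponent's health-zeroed event decrements it.
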(event `self.ReceiveBeginPlay`
  (`KismetSystemLibrary.K2_SetTimerDelegate` (delegate `Spawn`) 3.0 true))

(event `Spawn`
  (if (<= (`self.SpawnedActors`) 0)
    (for _array_element (`self.Spawners`)
      (`/Engine/EditorBlueprintResources/StandardMacros.IsValid` _array_element
        (:`Is Valid`
          (bind _returnvalue (`/Game/NecroPixelsContent/AI/BP_Spawner.SpawnActor` _array_element))
          (set `self.SpawnedActors` (+ (`self.SpawnedActors`) 1))
          (bind _returnvalue_2 (`self.GetComponentByClass` _returnvalue "/Game/NecroPixelsContent/Components/Pawns/HealthComponent.HealthComponent_C"))
          (`/Engine/EditorBlueprintResources/StandardMacros.IsValid` _returnvalue_2
            (:`Is Valid`
              (add `/Game/NecroPixelsContent/Components/Pawns/HealthComponent.OnHealthZeroed` _returnvalue_2 (delegate `OnHealthZeroed`)))))))))

(event `OnHealthZeroed`
  (set `self.SpawnedActors` (- (`self.SpawnedActors`) 1)))

(fn `UserConstructionScript`)