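; A perk vending machine that lets players spend score points to gain a perk effect.
; Its construction script looks up the perk name in DT_PerkList to set effect class, cost, and the flipbook sprite with a shadow copy.
; An overlap box registers it with the pawn's InteractComponent, which can show its purchase prompt.
; On interaction it checks the pawn's EffectsComponent can accept the perk, then deducts score from the PlayerState's ScoreComponent before adding it.
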(event `self.Box.OnComponentBeginOverlap`
  (params (OverlappedComponent :type "PrimitiveComponent Object Reference") (OtherActor :type "Actor Object Reference") (OtherComp :type "PrimitiveComponent Object Reference") (OtherBodyIndex :type Integer) (bFromSweep :type Boolean) (SweepResult :type "HitResult Structure (by ref)"))
  (bind _returnvalue (`self.GetComponentByClass` OtherActor "/Game/NecroPixelsContent/Components/InteractComponent.InteractComponent_C"))
  (`/Engine/EditorBlueprintResources/StandardMacros.IsValid` OtherActor
    (:`Is Valid`
      (`/Engine/EditorBlueprintResources/StandardMacros.IsValid` _returnvalue
        (:`Is Valid`
          (`/Game/NecroPixelsContent/Components/InteractComponent.SetInteractibleActor` _returnvalue self))))))

(event `self.Box.OnComponentEndOverlap`
  (params (OverlappedComponent :type "PrimitiveComponent Object Reference") (OtherActor :type "Actor Object Reference") (OtherComp :type "PrimitiveComponent Object Reference") (OtherBodyIndex :type Integer))
  (bind _returnvalue (`self.GetComponentByClass` OtherActor "/Game/NecroPixelsContent/Components/InteractComponent.InteractComponent_C"))
  (`/Engine/EditorBlueprintResources/StandardMacros.IsValid` OtherActor
    (:`Is Valid`
      (`/Engine/EditorBlueprintResources/StandardMacros.IsValid` _returnvalue
        (:`Is Valid`
          (`/Game/NecroPixelsContent/Components/InteractComponent.SetInteractibleActor` _returnvalue null))))))

(event `/Game/NecroPixelsContent/Interfaces/InteractInterface.InteractedWith`
  (params (OtherActor :type "Actor Object Reference"))
  (bind _aspawn (cast `Pawn` OtherActor))
  (bind _returnvalue (`self.GetComponentByClass` (`Pawn.PlayerState` _aspawn) "/Game/NecroPixelsContent/Components/ScoreComponent.ScoreComponent_C"))
  (`/Engine/EditorBlueprintResources/StandardMacros.IsValid` _returnvalue
    (:`Is Valid`
      (bind _returnvalue_2 (`self.GetComponentByClass` _aspawn "/Game/NecroPixelsContent/Components/EffectsComponent.EffectsComponent_C"))
      (`/Engine/EditorBlueprintResources/StandardMacros.IsValid` _returnvalue_2
        (:`Is Valid`
          (bind _bcanadd (`/Game/NecroPixelsContent/Components/EffectsComponent.CheckCanAddEffect` _returnvalue_2 (`self.PerkEffectClass`)))
          (if _bcanadd
            (bind _returnvalue_3 (`/Game/NecroPixelsContent/Components/ScoreComponent.TryRemoveScore` _returnvalue (`self.PerkCost`)))
            (if _returnvalue_3
              (`/Game/NecroPixelsContent/Components/EffectsComponent.AddEffect` _returnvalue_2 (`self.PerkEffectClass`)))))))))

(fn `GetInteractionInfo`
  (returns (DisplayString :type String))
  (return (`KismetTextLibrary.Conv_TextToString` (`|FormatText` "{Verb} {Noun} {Args}" "Purchase" (`KismetTextLibrary.Conv_NameToText` (`self.PerkName`)) (`|FormatText` "for {Perk Cost} points." (`self.PerkCost`))))))

(fn `UserConstructionScript`
  (bind _returnvalue (`|GetDataTableRow` "/Game/NecroPixelsContent/Perks/DT_PerkList.DT_PerkList" (`self.PerkName`))
    (:`then`
      (bind (_perkflipbook _perkeffectclass _perkcost) (break `/Game/NecroPixelsContent/Perks/ST_PerkListRow` _returnvalue))
      (set `self.PerkEffectClass` _perkeffectclass)
      (set `self.PerkCost` _perkcost)
      (`|ExecutionSequence`
        (:`then_0`
          (`PaperFlipbookComponent.SetFlipbook` (`self.PaperFlipbook`) _perkflipbook)
          (`SceneComponent.K2_SetRelativeLocation` (`self.PaperFlipbook`) (`KismetMathLibrary.MakeVector` 0.0 (- 0.0 (`self.SpriteYOffset`)) -14.0) false false))
        (:`then_1`
          (`PaperFlipbookComponent.SetFlipbook` (`self.PaperFlipbook_Shadow`) _perkflipbook)
          (`SceneComponent.K2_SetRelativeLocation` (`self.PaperFlipbook_Shadow`) (`KismetMathLibrary.MakeVector` 0.0 14.0 (`self.SpriteYOffset`)) false false))))))