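; BP_Door is an interactable door that triggers level travel.
; Its box collision registers the door as the interactible actor on an overlapping actor's InteractComponent and clears it when the overlap ends.
; On interaction, it passes the interacting actor to LevelTransition's LevelTravel, and its interaction info text is empty.
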(event `/Game/NecroPixelsContent/Interfaces/InteractInterface.InteractedWith`
  (params (OtherActor :type "Actor Object Reference"))
  (`/Game/NecroPixelsContent/Components/Gamemodes/LevelTransitionComponent.LevelTravel` (`self.LevelTransition`) OtherActor))

(event `self.Box_Collision.OnComponentBeginOverlap`
  (params (OverlappedComponent :type "PrimitiveComponent Object Reference") (OtherActor :type "Actor Object Reference") (OtherComp :type "PrimitiveComponent Object Reference") (OtherBodyIndex :type Integer) (bFromSweep :type Boolean) (SweepResult :type "HitResult Structure (by ref)"))
  (bind _returnvalue (`self.GetComponentByClass` OtherActor "/Game/NecroPixelsContent/Components/Pawns/InteractComponent.InteractComponent_C"))
  (`/Engine/EditorBlueprintResources/StandardMacros.IsValid` _returnvalue
    (:`Is Valid`
      (`/Game/NecroPixelsContent/Components/Pawns/InteractComponent.SetInteractibleActor` _returnvalue self))))

(event `self.Box_Collision.OnComponentEndOverlap`
  (params (OverlappedComponent :type "PrimitiveComponent Object Reference") (OtherActor :type "Actor Object Reference") (OtherComp :type "PrimitiveComponent Object Reference") (OtherBodyIndex :type Integer))
  (bind _returnvalue (`self.GetComponentByClass` OtherActor "/Game/NecroPixelsContent/Components/Pawns/InteractComponent.InteractComponent_C"))
  (`/Engine/EditorBlueprintResources/StandardMacros.IsValid` _returnvalue
    (:`Is Valid`
      (`/Game/NecroPixelsContent/Components/Pawns/InteractComponent.SetInteractibleActor` _returnvalue null))))

(fn `GetInteractionInfo`
  (returns (DisplayString :type String))
  (return ""))

(fn `UserConstructionScript`)