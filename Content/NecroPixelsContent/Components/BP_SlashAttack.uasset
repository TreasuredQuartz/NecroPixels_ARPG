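; BP_SlashAttack is a short-lived slash hitbox actor that deals fixed damage to overlapped actors with a HealthComponent.
; It records each hit actor in OverlappedActors so none is damaged twice by the same slash.
; A brief lifespan set on BeginPlay removes it, as the flipbook-finished handler that would hide and destroy it is never bound.
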(event `self.ReceiveBeginPlay`
  (`self.SetLifeSpan` 0.2))

(event `OnFinishedPlaying`
  (`self.SetActorHiddenInGame` true)
  (`self.K2_DestroyActor`))

(event `self.ReceiveActorBeginOverlap`
  (params (OtherActor :type "Actor Object Reference"))
  (bind _returnvalue (`self.GetComponentByClass` OtherActor "/Game/NecroPixelsContent/Components/HealthComponent.HealthComponent_C"))
  (`/Engine/EditorBlueprintResources/StandardMacros.IsValid` _returnvalue
    (:`Is Valid`
      (if (not (`KismetArrayLibrary.Array_Contains` (`self.OverlappedActors`) OtherActor))
        (`KismetArrayLibrary.Array_Add` (`self.OverlappedActors`) OtherActor)
        (`/Game/NecroPixelsContent/Components/HealthComponent.DealDamage` _returnvalue 50.0)))))

(fn `UserConstructionScript`)