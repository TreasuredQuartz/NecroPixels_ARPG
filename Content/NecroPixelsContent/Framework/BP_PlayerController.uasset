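; Player controller that manages the local player's scoreboard and pause menu widgets.
; On BeginPlay it creates both widgets, adds them to the player screen and sets game-only input.
; Enhanced Input actions show the scoreboard while triggered and hide it on completion.
; The pause action reveals the menu and switches to UI-only input focused on it, without pausing the game or handling resume here.
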(event `self.ReceiveBeginPlay`
  (`parent.ReceiveBeginPlay`)
  (`|ExecutionSequence`
    (:`then_0`
      (bind _returnvalue (`|CreateWidget` "/Game/NecroPixelsContent/UI/Scoreboard/WBP_Scoreboard.WBP_Scoreboard_C" self))
      (set `self.ScoreboardWidget` _returnvalue)
      (`UserWidget.AddToPlayerScreen` _returnvalue 0)
      (`WidgetBlueprintLibrary.SetInputMode_GameOnly` self))
    (:`then_1`
      (bind _returnvalue_2 (`|CreateWidget` "/Game/NecroPixelsContent/UI/Menus/WBP_PauseMenu.WBP_PauseMenu_C"))
      (bind _output_get (set `self.PauseMenu` _returnvalue_2))
      (`UserWidget.AddToPlayerScreen` _output_get 0))))

(event `EnhancedInput|/Game/NecroPixelsContent/Input/IA_Scoreboard`
  (params (ActionValue :type Boolean) (ElapsedSeconds :type "Float (double-precision)") (TriggeredSeconds :type "Float (double-precision)") (InputAction :type "InputAction Object Reference" :default "/Game/NecroPixelsContent/Input/IA_Scoreboard.IA_Scoreboard"))
  (:`Triggered`
    (`Widget.SetVisibility` (`self.ScoreboardWidget`) "HitTestInvisible"))
  (:`Completed`
    (`Widget.SetVisibility` (`self.ScoreboardWidget`) "Hidden")))

(event `EnhancedInput|/Game/NecroPixelsContent/Input/IA_Pause`
  (params (ActionValue :type Boolean) (ElapsedSeconds :type "Float (double-precision)") (TriggeredSeconds :type "Float (double-precision)") (InputAction :type "InputAction Object Reference" :default "/Game/NecroPixelsContent/Input/IA_Pause.IA_Pause"))
  (:`Triggered`
    (`Widget.SetVisibility` (`self.PauseMenu`) "SelfHitTestInvisible")
    (`WidgetBlueprintLibrary.SetInputMode_UIOnlyEx` self (`self.PauseMenu`))))

(fn `UserConstructionScript`)