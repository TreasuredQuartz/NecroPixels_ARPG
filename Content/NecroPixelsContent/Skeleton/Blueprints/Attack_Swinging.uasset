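; Attack_Swinging is a short-lived damage actor for the Skeleton's swinging melee attack, expiring after one second.
; On overlap it ignores its owner and records each actor in OverlappedActors so each is hit only once.
; Each hit applies fixed blunt-force damage credited to the instigator's controller.
; Targets with a CharacterMovementComponent also receive a force along the attack's forward vector with a slight upward term.
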(event `self.ReceiveBeginPlay`
  (`self.SetLifeSpan` 1.0))

(event `self.ReceiveActorBeginOverlap`
  (params (OtherActor :type "Actor Object Reference"))
  (bind _returnvalue (`self.GetComponentByClass` OtherActor "/Script/Engine.CharacterMovementComponent"))
  (if (!= OtherActor (`self.GetOwner`))
    (if (not (`KismetArrayLibrary.Array_Contains` (`self.OverlappedActors`) OtherActor))
      (`KismetArrayLibrary.Array_Add` (`self.OverlappedActors`) OtherActor)
      (`GameplayStatics.ApplyDamage` OtherActor 50.0 (`self.GetInstigatorController`) self "/Game/NecroPixelsContent/DamageTypes/DmgType_BluntForce.DmgType_BluntForce_C")
      (`/Engine/EditorBlueprintResources/StandardMacros.IsValid` _returnvalue
        (:`Is Valid`
          (`CharacterMovementComponent.AddForce` _returnvalue (+ (* (`self.GetActorForwardVector`) (`self.ForceApplied`)) (* (0.0 0.0 1.0) 1000.0))))))))

(fn `UserConstructionScript`
  (`parent.UserConstructionScript`))