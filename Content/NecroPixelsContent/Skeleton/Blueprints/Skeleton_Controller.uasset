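; Skeleton_Controller is the AI controller for skeleton enemies.
; On BeginPlay it runs the BT_Horde behavior tree and sets the player character as the blackboard target.
; It binds to the controlled pawn's HealthComponent, if present, and stops the brain's logic when health reaches zero.
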(event `self.ReceiveBeginPlay`
  (bind _returnvalue (`self.K2_GetPawn`))
  (bind _returnvalue_2 (`self.GetComponentByClass` _returnvalue "/Game/NecroPixelsContent/Components/HealthComponent.HealthComponent_C"))
  (`self.RunBehaviorTree` "/Game/NecroPixelsContent/AI/BT_Horde.BT_Horde")
  (`BlackboardComponent.SetValueAsObject` (`AIBlueprintHelperLibrary.GetBlackboard` null) (`self.TargetKey`) (`GameplayStatics.GetPlayerCharacter` 0))
  (`/Engine/EditorBlueprintResources/StandardMacros.IsValid` _returnvalue
    (:`Is Valid`
      (`/Engine/EditorBlueprintResources/StandardMacros.IsValid` _returnvalue_2
        (:`Is Valid`
          (add `/Game/NecroPixelsContent/Components/HealthComponent.OnHealthZeroed` _returnvalue_2 (delegate `OnDeath`)))))))

(event `OnDeath`
  (`BrainComponent.StopLogic` (`self.BrainComponent`) "Death"))

(fn `UserConstructionScript`)