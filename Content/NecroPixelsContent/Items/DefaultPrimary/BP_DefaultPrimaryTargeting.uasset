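; Targeting actor for the default primary item that positions itself around its owner according to the mouse cursor.
; On BeginPlay it caches the instigator's PlayerController.
; Each tick it converts the cursor's offset from viewport center into a ratio, scales and clamps it by TargetingRange, then teleports to the owner's location plus that offset.
; IA_Look input separately stores a normalized DesiredDirection, which this graph does not use for positioning.
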(event `EnhancedInput|/Game/NecroPixelsContent/Input/IA_Look`
  (params (ActionValue :type "Vector2D Structure") (ElapsedSeconds :type "Float (double-precision)") (TriggeredSeconds :type "Float (double-precision)") (InputAction :type "InputAction Object Reference" :default "/Game/NecroPixelsContent/Input/IA_Look.IA_Look"))
  (bind _returnvalue (`KismetMathLibrary.Normal2D` ActionValue))
  (:`Triggered`
    (if (!= (`KismetMathLibrary.VSize2D` _returnvalue) 0.0)
      (set `self.DesiredDirection` _returnvalue))))

(event `self.ReceiveBeginPlay`
  (`parent.ReceiveBeginPlay`)
  (bind _asplayer_controller (cast `PlayerController` (`self.GetInstigatorController`)))
  (set `self.OwnerController` _asplayer_controller))

(event `self.ReceiveTick`
  (params (DeltaSeconds :type "Float (single-precision)"))
  (`self.SetTargetingOffset`)
  (`self.K2_SetActorLocation` (+ (`self.TargetingOffset`) (`self.K2_GetActorLocation` (`self.GetOwner`))) false true))

(fn `SetTargetingOffset`
  (locals (LocHalfViewportSize :type "Vector2D Structure") (LocRealMousePosition :type "Vector2D Structure") (LocMousePosRatio :type "Vector2D Structure"))
  (bind (_lochalfviewportsize_x _lochalfviewportsize_y) (`KismetMathLibrary.BreakVector2D` (`local.LocHalfViewportSize`)))
  (bind (_locrealmouseposition_x _locrealmouseposition_y) (`KismetMathLibrary.BreakVector2D` (`local.LocRealMousePosition`)))
  (bind (_lochalfviewportsize_x_2 _lochalfviewportsize_y_2) (`KismetMathLibrary.BreakVector2D` (`local.LocHalfViewportSize`)))
  (bind (_locmouseposratio_x _locmouseposratio_y) (`KismetMathLibrary.BreakVector2D` (`local.LocMousePosRatio`)))
  (bind _targetingrange (`self.TargetingRange`))
  (bind _targetingrange_2 (`self.TargetingRange`))
  (bind (_locationx _locationy) (`PlayerController.GetMousePosition` (`self.OwnerController`)))
  (bind (_sizex _sizey) (`PlayerController.GetViewportSize` (`self.OwnerController`)))
  (set `local.LocHalfViewportSize` (`KismetMathLibrary.MakeVector2D` (/ _sizex 2) (/ _sizey 2)))
  (set `local.LocRealMousePosition` (`KismetMathLibrary.MakeVector2D` (- _locationx _lochalfviewportsize_x) (- _locationy _lochalfviewportsize_y)))
  (set `local.LocMousePosRatio` (`KismetMathLibrary.MakeVector2D` (/ _locrealmouseposition_x _lochalfviewportsize_x_2) (/ _locrealmouseposition_y _lochalfviewportsize_y_2)))
  (set `self.TargetingOffset` (`KismetMathLibrary.ClampVectorSize` (`KismetMathLibrary.MakeVector` (* _locmouseposratio_x _targetingrange) (* _locmouseposratio_y _targetingrange)) (- 0.0 _targetingrange_2) _targetingrange_2))
  (return))

(fn `UserConstructionScript`
  (`parent.UserConstructionScript`))