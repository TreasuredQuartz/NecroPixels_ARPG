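; BP_PowerSwitch is an interactable switch that toggles power generation in the level.
; Overlapping actors with an InteractComponent register the switch as their interactible target and clear it on leaving.
; Interaction passes through a gate, toggles the PowerGeneratorComponent, swaps the on/off sprite and plays a sound.
; The gate closes after each use and a one-second timer is set, acting as a cooldown against repeated presses.
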(event `self.ReceiveActorBeginOverlap`
  (params (OtherActor :type "Actor Object Reference"))
  (bind _returnvalue (`self.GetComponentByClass` OtherActor "/Game/NecroPixelsContent/Components/Pawns/InteractComponent.InteractComponent_C"))
  (`/Engine/EditorBlueprintResources/StandardMacros.IsValid` OtherActor
    (:`Is Valid`
      (`/Engine/EditorBlueprintResources/StandardMacros.IsValid` _returnvalue
        (:`Is Valid`
          (`/Game/NecroPixelsContent/Components/Pawns/InteractComponent.SetInteractibleActor` _returnvalue self))))))

(event `self.ReceiveActorEndOverlap`
  (params (OtherActor :type "Actor Object Reference"))
  (bind _returnvalue (`self.GetComponentByClass` OtherActor "/Game/NecroPixelsContent/Components/Pawns/InteractComponent.InteractComponent_C"))
  (`/Engine/EditorBlueprintResources/StandardMacros.IsValid` OtherActor
    (:`Is Valid`
      (`/Engine/EditorBlueprintResources/StandardMacros.IsValid` _returnvalue
        (:`Is Valid`
          (`/Game/NecroPixelsContent/Components/Pawns/InteractComponent.SetInteractibleActor` _returnvalue null))))))

(event `/Game/NecroPixelsContent/Interfaces/InteractInterface.InteractedWith`
  (params (OtherActor :type "Actor Object Reference"))
  (`/Engine/EditorBlueprintResources/StandardMacros.FlipFlop`
    (:`A`
      _)
    (:`B`
      _))
  (`/Engine/EditorBlueprintResources/StandardMacros.Gate` false :!label _label
    (:`Exit`
      (`self.PreventInteraction`)
      (`/Game/NecroPixelsContent/Components/PowerGeneratorComponent.TogglePower` (`self.PowerGeneratorComponent`))
      (`PaperSpriteComponent.SetSprite` (`self.Sprite_PowerSwitch`) (select `bool` (`/Game/NecroPixelsContent/Components/PowerGeneratorComponent.bIsGeneratingPower` (`self.PowerGeneratorComponent`)) :`false` "/Game/NecroPixelsContent/Enviornment/PowerSwitch/Sprite_PowerSwitch_Off.Sprite_PowerSwitch_Off" :`true` "/Game/NecroPixelsContent/Enviornment/PowerSwitch/Sprite_PowerSwitch_On.Sprite_PowerSwitch_On" :!type "PaperSprite Object Reference"))
      (`AudioComponent.Play` (`self.Audio`) 0.0)
      (`KismetSystemLibrary.K2_SetTimerDelegate` (`|CreateDelegate` :!event `AllowInteraction`) 1.0))))

(event `AllowInteraction`
  (goto _label :!via `Open`))

(event `PreventInteraction`
  (goto _label :!via `Close`))

(fn `GetInteractionInfo`
  (returns (DisplayString :type String))
  (return "Turn the power on..."))

(fn `UserConstructionScript`)