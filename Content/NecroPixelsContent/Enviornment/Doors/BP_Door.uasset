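; BP_Door is a purchasable door that the player opens by spending score points.
; Its Interact_Box overlap registers or clears the door on the overlapping actor's InteractComponent and supplies a hold-to-open prompt showing the Cost.
; On interaction, it asks the ScoreComponent on the instigator controller's PlayerState to remove the Cost, and if that succeeds it disables collision and destroys itself.
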(event `self.Interact_Box.OnComponentBeginOverlap`
  (params (OverlappedComponent :type "PrimitiveComponent Object Reference") (OtherActor :type "Actor Object Reference") (OtherComp :type "PrimitiveComponent Object Reference") (OtherBodyIndex :type Integer) (bFromSweep :type Boolean) (SweepResult :type "HitResult Structure (by ref)"))
  (bind _returnvalue (`self.GetComponentByClass` OtherActor "/Game/NecroPixelsContent/Components/InteractComponent.InteractComponent_C"))
  (`/Engine/EditorBlueprintResources/StandardMacros.IsValid` _returnvalue
    (:`Is Valid`
      (`/Game/NecroPixelsContent/Components/InteractComponent.SetInteractibleActor` _returnvalue self))))

(event `self.Interact_Box.OnComponentEndOverlap`
  (params (OverlappedComponent :type "PrimitiveComponent Object Reference") (OtherActor :type "Actor Object Reference") (OtherComp :type "PrimitiveComponent Object Reference") (OtherBodyIndex :type Integer))
  (bind _returnvalue (`self.GetComponentByClass` OtherActor "/Game/NecroPixelsContent/Components/InteractComponent.InteractComponent_C"))
  (`/Engine/EditorBlueprintResources/StandardMacros.IsValid` _returnvalue
    (:`Is Valid`
      (`/Game/NecroPixelsContent/Components/InteractComponent.SetInteractibleActor` _returnvalue null))))

(event `/Game/NecroPixelsContent/Interfaces/InteractInterface.InteractedWith`
  (params (OtherActor :type "Actor Object Reference"))
  (bind _playerstate (`Controller.PlayerState` (`self.GetInstigatorController` OtherActor)))
  (bind _returnvalue (`self.GetComponentByClass` _playerstate "/Game/NecroPixelsContent/Components/ScoreComponent.ScoreComponent_C"))
  (`/Engine/EditorBlueprintResources/StandardMacros.IsValid` _playerstate
    (:`Is Valid`
      (`/Engine/EditorBlueprintResources/StandardMacros.IsValid` _returnvalue
        (:`Is Valid`
          (bind _returnvalue_2 (`/Game/NecroPixelsContent/Components/ScoreComponent.TryRemoveScore` _returnvalue (`self.Cost`)))
          (if _returnvalue_2
            (`self.SetActorEnableCollision` false)
            (`self.K2_DestroyActor`)))))))

(fn `GetInteractionInfo`
  (returns (DisplayString :type String))
  (return (`KismetTextLibrary.Conv_TextToString` (`|FormatText` "Hold {Interact} To Open Door [{Cost} Points]" _ (`self.Cost`)))))

(fn `UserConstructionScript`)